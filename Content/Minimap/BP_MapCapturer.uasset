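; BP_MapCapturer is a minimap scene-capture actor that renders tagged actors into a supplied render target, working only on non-authority clients.
; BeginPlay fills the show-only list from MiniMapVisible-tagged actors and enables custom depth on their static meshes.
; Initialize assigns the target, sets every-frame capture from a saved GameInstance setting, then captures after a short delay and disables custom depth.
; The looping capture timer is unconnected.
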(event `self.ReceiveBeginPlay`
  (`/Engine/EditorBlueprintResources/ActorMacros.Switch Has Authority`
    (:`Remote`
      (bind _outactors (`GameplayStatics.GetAllActorsWithTag` "MiniMapVisible"))
      (set `SceneCaptureComponent.ShowOnlyActors` _outactors (`self.CaptureComponent2D`))
      (`self.SetAllStencilValues` true))))

(event `self.ReceiveTick`
  (params (DeltaSeconds :type "Float (single-precision)")))

(event `Initialize`
  (params (`Texture Target` :type "TextureRenderTarget2D Object Reference"))
  (`/Engine/EditorBlueprintResources/ActorMacros.Switch Has Authority`
    (:`Remote`
      (`self.OnCaptureEveryFrameUpdated`)
      (set `SceneCaptureComponent2D.TextureTarget` `Texture Target` (`self.CaptureComponent2D`))
      (`KismetSystemLibrary.Delay` 0.2)
      (`SceneCaptureComponent2D.CaptureScene` (`self.CaptureComponent2D`))
      (`self.SetAllStencilValues` false))))

(event `OnCaptureEveryFrameUpdated`
  (bind _value (message `/Game/Blueprints/Interfaces/BPI_Menu.GetSaveDynamiclyUpdateMinimap` (`GameplayStatics.GetGameInstance`)))
  (set `SceneCaptureComponent.bCaptureEveryFrame` _value (`self.CaptureComponent2D`)))

(event `Capture`
  (`SceneCaptureComponent2D.CaptureScene` (`self.CaptureComponent2D`)))

(fn `SetAllStencilValues`
  (params (Enabled :type Boolean))
  (for _array_element (`SceneCaptureComponent.ShowOnlyActors` (`self.CaptureComponent2D`))
    (for _array_element_2 (`self.K2_GetComponentsByClass` _array_element "/Script/Engine.StaticMeshComponent")
      (`PrimitiveComponent.SetRenderCustomDepth` _array_element_2 Enabled))))

(fn `UserConstructionScript`)