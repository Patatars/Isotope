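; Blueprint function library for the game's video options: display resolution, brightness and graphics settings, plus a getter for the save-game slot name.
; SetVideoSettings switches on the option type, maps an index to Game User Settings values or console commands, and returns a display label.
; Resolution helpers fill an option list with "WxH" strings and parse them back, while brightness runs the gamma console command.
; None of these functions calls ApplySettings or saves.
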(fn `GetAllDisplayResolutions`
  (params (Target :type "ComboBoxString Object Reference"))
  (bind _resolutions (`KismetSystemLibrary.GetSupportedFullscreenResolutions`))
  (for _array_element _resolutions
    (bind (_x _y) (break `IntPoint` _array_element))
    (`ComboBoxString.AddOption` Target (`KismetStringLibrary.Concat_StrStr` (`KismetStringLibrary.Conv_IntToString` _x) "x" (`KismetStringLibrary.Conv_IntToString` _y)))))

(fn `SetBrightness`
  (params (Brightness :type "Float (double-precision)"))
  (returns (OutputPin :type String))
  (bind _returnvalue (`KismetStringLibrary.Concat_StrStr` "gamma " (`KismetStringLibrary.Conv_DoubleToString` (* (`KismetMathLibrary.MapRangeClamped` Brightness 0.0 1.0 0.0 1.0) 5.0))))
  (`KismetSystemLibrary.ExecuteConsoleCommand` null _returnvalue null)
  (return _returnvalue))

(fn `SetResolutions`
  (params (Text :type Text))
  (bind (_lefts _rights) (`KismetStringLibrary.Split` (`KismetTextLibrary.Conv_TextToString` Text) "x"))
  (bind _returnvalue (`GameUserSettings.GetGameUserSettings`))
  (`GameUserSettings.SetScreenResolution` _returnvalue (make `IntPoint` (`KismetStringLibrary.Conv_StringToInt` _lefts) (`KismetStringLibrary.Conv_StringToInt` _rights)))
  (return))

(fn `SetVideoSettings`
  (params (`Select Settings Options` :type "/Game/MGS_vs_DownGrade/Blueprint/EVideoSettings Enum" :default "NewEnumerator1") (Index :type Integer))
  (returns (Text :type Text))
  (locals (ForText :type Text))
  (bind _returnvalue (select `int` Index :`0` 0 :`1` 1 :`2` 2 :`3` 3 :`4` 4))
  (bind _returnvalue_2 (select `int` Index :`0` 0 :`1` 1 :`2` 2 :`3` 3 :`4` 4))
  (bind _returnvalue_3 (select `int` Index :`0` 0 :`1` 1 :`2` 2 :`3` 3 :`4` 4))
  (switch `/Game/MGS_vs_DownGrade/Blueprint/EVideoSettings` `Select Settings Options`
    (:`NewEnumerator1`
      (bind _returnvalue_4 (`GameUserSettings.GetGameUserSettings`))
      (`GameUserSettings.SetFullscreenMode` _returnvalue_4 (select `int` Index :`0` "Fullscreen" :`1` "WindowedFullscreen" :`2` "Windowed" :!type "EWindowMode Enum"))
      (set `local.ForText` (select `int` Index :`0` "FULLSCREEN" :`1` "BORDERLESS" :`2` "WINDOWED" :!type "Text")))
    (:`NewEnumerator2`
      (bind _returnvalue_5 (`GameUserSettings.GetGameUserSettings`))
      (`GameUserSettings.SetAntiAliasingQuality` _returnvalue_5 (select `int` Index :`0` 4 :`1` 0))
      (set `local.ForText` (select `int` Index :`0` "YES" :`1` "NO" :!type "Text")))
    (:`NewEnumerator3`
      (`KismetSystemLibrary.ExecuteConsoleCommand` null (`KismetStringLibrary.Concat_StrStr` "r.DefaultFeature.AntiAliasing " (select `int` Index :`0` "0" :`1` "1" :`2` "2" :`3` "3")) null)
      (set `local.ForText` (select `int` Index :`0` "NONE" :`1` "FXAA" :`2` "TXAA" :`3` "MSAA" :!type "Text")))
    (:`NewEnumerator4`
      (bind _returnvalue_6 (`GameUserSettings.GetGameUserSettings`))
      (`GameUserSettings.SetVSyncEnabled` _returnvalue_6 (select `int` Index :`0` true :`1` false))
      (set `local.ForText` (select `int` Index :`0` "YES" :`1` "NO" :!type "Text")))
    (:`NewEnumerator5`
      (bind _returnvalue_7 (`GameUserSettings.GetGameUserSettings`))
      (`GameUserSettings.SetFrameRateLimit` _returnvalue_7 (select `int` Index :`0` 30.0 :`1` 60.0 :`2` 120.0 :`3` 0.0))
      (set `local.ForText` (select `int` Index :`0` "30 FPS" :`1` "60 FPS" :`2` "120 FPS" :`3` "VARIABLE" :!type "Text")))
    (:`NewEnumerator6`
      (switch `int` Index
        (:`0`
          (`KismetSystemLibrary.ExecuteConsoleCommand` null "r.MotionBlur.Amount 4" null)
          (`KismetSystemLibrary.ExecuteConsoleCommand` null "r.MotionBlurQuality 4" null)
          (set `local.ForText` "YES"))
        (:`1`
          (`KismetSystemLibrary.ExecuteConsoleCommand` null "r.MotionBlur.Amount 0" null)
          (`KismetSystemLibrary.ExecuteConsoleCommand` null "r.MotionBlurQuality 0" null)
          (set `local.ForText` "NO"))))
    (:`NewEnumerator7`
      (bind _returnvalue_8 (`GameUserSettings.GetGameUserSettings`))
      (`GameUserSettings.SetTextureQuality` _returnvalue_8 _returnvalue)
      (`GameUserSettings.SetShadowQuality` _returnvalue_8 _returnvalue)
      (set `local.ForText` (select `int` Index :`0` "LOW" :`1` "STANDARD" :`2` "HIGH" :`3` "ULTRA" :`4` "HYPER" :!type "Text"))
      (bind _returnvalue_9 (`GameUserSettings.GetGameUserSettings`))
      (`GameUserSettings.SetResolutionScaleValueEx` _returnvalue_9 100.0))
    (:`NewEnumerator8`
      (bind _returnvalue_10 (`GameUserSettings.GetGameUserSettings`))
      (`GameUserSettings.SetPostProcessingQuality` _returnvalue_10 _returnvalue_2)
      (`GameUserSettings.SetVisualEffectQuality` _returnvalue_10 _returnvalue_2)
      (set `local.ForText` (select `int` Index :`0` "LOW" :`1` "STANDARD" :`2` "HIHG" :`3` "ULTRA" :`4` "HYPER" :!type "Text")))
    (:`NewEnumerator9`
      (bind _returnvalue_11 (`GameUserSettings.GetGameUserSettings`))
      (`GameUserSettings.SetViewDistanceQuality` _returnvalue_11 _returnvalue_3)
      (`GameUserSettings.SetFoliageQuality` _returnvalue_11 _returnvalue_3)
      (set `local.ForText` (select `int` Index :`0` "MINIMUM" :`1` "NORMAL" :`2` "MAXIMUM" :`3` "OVERLY" :`4` "EXCESSIVE" :!type "Text"))))
  (return (`local.ForText`)))

(fn `SlotNameSaveGame`
  (returns (NameSlot_ :type String))
  (locals (NameSlot :type String :default "Settings/Video"))
  (return (`local.NameSlot`)))