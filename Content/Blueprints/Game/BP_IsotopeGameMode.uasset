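; Game mode for a team isotope-collection match, where holding the winning score through a countdown ends the game.
; Isotope pickups and losses adjust the player's and team's scores, and a death updates kill stats and removes the victim's whole score.
; Each change rechecks the top team score, starting an end timer at the threshold or cancelling it below.
; When the timer expires, the current top team is passed to EndGame.
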(event `/Game/Blueprints/Interfaces/BPI_IsotopeGameMode.IsotopeLoosed`
  (params (PlayerState :type "/Game/Blueprints/Player/BP_PlayerState Object Reference") (Count :type Integer))
  (`self.UpdateIsotopeCounter` PlayerState (* Count -1)))

(event `/Game/Blueprints/Interfaces/BPI_IsotopeGameMode.IsotopeCollected`
  (params (PlayerState :type "/Game/Blueprints/Player/BP_PlayerState Object Reference") (Count :type Integer))
  (`self.UpdateIsotopeCounter` PlayerState Count))

(fn `CheckEndGame`
  (bind (_team _score) (`/Game/Blueprints/Game/BP_GameState.GetMaxScore` (`self.BP_GameState`)))
  (if (>= _score (`self.ScoreToWin`))
    (`self.CountdownToEnd`)
    (else
      (`self.ResetCountdownToEnd`))))

(fn `CountdownToEnd`
  (set `/Game/Blueprints/Game/BP_GameState.GameStatus` "NewEnumerator4" (`self.BP_GameState`))
  (if (not (`KismetSystemLibrary.K2_IsValidTimerHandle` (`self.TimerToEndGame`)))
    (bind _returnvalue (`KismetSystemLibrary.K2_SetTimer` null "TimerIsOver" (`KismetMathLibrary.Conv_IntToDouble` (`/Game/Blueprints/Game/BP_GameState.TimeBeforeEnd` (`self.BP_GameState`)))))
    (set `self.TimerToEndGame` _returnvalue)))

(fn `PlayerDied`
  (params (Killed :type "/Game/Blueprints/Player/BP_PlayerState Object Reference") (Died :type "/Game/Blueprints/Player/BP_PlayerState Object Reference"))
  (`self.UpdateKillStat` Killed Died)
  (`self.IsotopeLoosed` (`local.Died`) (`/Game/Blueprints/Player/BP_PlayerState.GetOwnScore` (`local.Died`))))

(fn `ResetCountdownToEnd`
  (set `/Game/Blueprints/Game/BP_GameState.GameStatus` "NewEnumerator1" (`self.BP_GameState`))
  (`KismetSystemLibrary.K2_ClearAndInvalidateTimerHandle` (`self.TimerToEndGame`)))

(fn `TimerIsOver`
  (bind _team (`/Game/Blueprints/Game/BP_GameState.GetMaxScore` (`self.BP_GameState`)))
  (`self.EndGame` _team))

(fn `UpdateIsotopeCounter`
  (params (PlayerState :type "/Game/Blueprints/Player/BP_PlayerState Object Reference") (Count :type Integer))
  (`/Game/Blueprints/Player/BP_PlayerState.AddOwnScore` PlayerState Count)
  (`/Game/Blueprints/Game/BP_GameState.AddScoreToTeam` (`self.BP_GameState`) (`/Game/Blueprints/Player/BP_PlayerState.Team` (`local.PlayerState`)) (`local.Count`))
  (`self.CheckEndGame`))

(fn `UserConstructionScript`
  (`parent.UserConstructionScript`))