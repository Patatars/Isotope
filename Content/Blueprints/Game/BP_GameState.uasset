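; Game state for team matches that tracks each team's players and score, plus a replicated game status.
; At BeginPlay it parses command-line Team1 and Team2 lists into a player-ID-to-team map.
; Team selection picks the smallest team in Development builds and otherwise looks up that map.
; Helper functions edit the Teams struct array, while dispatchers announce team joins, score sets and status changes.
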(event `self.ReceiveBeginPlay`
  (bind _returnvalue (`KismetSystemLibrary.GetCommandLine`))
  (bind _result (`self.GetPlayerToTeam` _returnvalue))
  (set `self.PlayerIdToTeam` _result))

(event `ScoreUpdated`
  (params (Team :type "/Game/Blueprints/Game/E_Teams Enum" :default "NewEnumerator0") (Score :type Integer))
  (`self.ScoreUpdatedDispatcher` Team Score))

(event `TeamChanged`
  (params (Team :type "/Game/Blueprints/Game/E_Teams Enum" :default "NewEnumerator0") (Player :type "/Game/Blueprints/Player/BP_PlayerState Object Reference") (Joined :type Boolean))
  (`self.TeamChangedDispatcher` Team Player Joined))

(fn `AddAllPlayersToTeam`
  (params (TargetMap :type "Map of String to /Game/Blueprints/Game/E_Teams Enum (by ref)") (Players :type String) (Value :type "/Game/Blueprints/Game/E_Teams Enum" :default "NewEnumerator0"))
  (for _array_element (`KismetStringLibrary.ParseIntoArray` Players ",")
    (`BlueprintMapLibrary.Map_Add` TargetMap _array_element Value)))

(fn `AddPlayerToTeam`
  (params (Team :type "/Game/Blueprints/Game/E_Teams Enum" :default "NewEnumerator0") (Player :type "/Game/Blueprints/Player/BP_PlayerState Object Reference"))
  (bind _player (`local.Player`))
  (`/Engine/EditorBlueprintResources/StandardMacros.IncrementInt` (`self.NumPlayers`)
    (:`  `
      (bind (_players _array_index) (`self.FindArrayToAdd` Team))
      (bind (_team _players_2 _score) (break `/Game/Blueprints/Game/ST_TeamPlayers` _players))
      (`KismetArrayLibrary.Array_Add` _players_2 (`local.Player`))
      (`KismetArrayLibrary.Array_Set` (`self.Teams`) _array_index (make `/Game/Blueprints/Game/ST_TeamPlayers` _team _players_2 _score))
      (bind _output_get (set `/Game/Blueprints/Player/BP_PlayerState.Team` (`local.Team`) _player))
      (`self.TeamChanged` _output_get _player true))))

(fn `AddScoreToTeam`
  (params (Team :type "/Game/Blueprints/Game/E_Teams Enum" :default "NewEnumerator0") (Score :type Integer))
  (bind (_players _array_index) (`self.FindArrayToAdd` Team))
  (bind (_team _players_2 _score) (break `/Game/Blueprints/Game/ST_TeamPlayers` _players))
  (`KismetArrayLibrary.Array_Set` (`self.Teams`) _array_index (make `/Game/Blueprints/Game/ST_TeamPlayers` _team _players_2 (+ _score (`local.Score`))))
  (return))

(fn `FindArrayToAdd`
  (params (Team :type "/Game/Blueprints/Game/E_Teams Enum" :default "NewEnumerator0"))
  (returns (Players :type "/Game/Blueprints/Game/ST_TeamPlayers Structure") (`Array Index` :type Integer))
  (bind _st_teamplayers (make `/Game/Blueprints/Game/ST_TeamPlayers` Team (`|MakeArray`)))
  (for (_array_element _array_index) (`self.Teams`)
    (if (`|EnumEquality` (`.Team_2_39BED99042296F9BED34488332509E17` (break `/Game/Blueprints/Game/ST_TeamPlayers` _array_element)) (`local.Team`))
      (return _array_element _array_index)))
  (bind _returnvalue (`KismetArrayLibrary.Array_Add` (`self.Teams`) _st_teamplayers))
  (return _st_teamplayers _returnvalue))

(fn `GetAllPawns`
  (returns (Pawns :type "Array of Pawn Object Reference"))
  (locals (Result :type "Array of Pawn Object Reference"))
  (for _array_element (`self.Teams`)
    (for _array_element_2 (`.Players_6_17086216468522D98153889462D27349` (break `/Game/Blueprints/Game/ST_TeamPlayers` _array_element))
      (`/Engine/EditorBlueprintResources/StandardMacros.IsValid` _array_element_2
        (:`Is Valid`
          (bind _returnvalue (`PlayerState.GetPawn` _array_element_2))
          (`/Engine/EditorBlueprintResources/StandardMacros.IsValid` _returnvalue
            (:`Is Valid`
              (`KismetArrayLibrary.Array_Add` (`local.Result`) _returnvalue))))))
    (return (`local.Result`))))

(fn `GetMaxScore`
  (returns (Team :type "/Game/Blueprints/Game/E_Teams Enum") (Score :type Integer))
  (locals (MaxTeam :type "/Game/Blueprints/Game/E_Teams Enum") (MaxScore :type Integer))
  (bind (_team _players _score) (break `/Game/Blueprints/Game/ST_TeamPlayers` (`|GetArrayItem` (`self.Teams`))))
  (set `local.MaxTeam` _team)
  (set `local.MaxScore` _score)
  (for _array_element (`self.Teams`)
    (bind (_team_2 _players_2 _score_2) (break `/Game/Blueprints/Game/ST_TeamPlayers` _array_element))
    (if (> _score_2 (`local.MaxScore`))
      (set `local.MaxScore` _score_2)
      (set `local.MaxTeam` _team_2)))
  (return (`local.MaxTeam`) (`local.MaxScore`)))

(fn `GetPlayerToTeam`
  (params (Input :type String))
  (returns (Result :type "Map of String to /Game/Blueprints/Game/E_Teams Enum"))
  (locals (Result :type "Map of String to /Game/Blueprints/Game/E_Teams Enum"))
  (bind (_outtokens _outswitches _outparams) (`KismetSystemLibrary.ParseCommandLine` Input))
  (`self.AddAllPlayersToTeam` (`local.Result`) (`BlueprintMapLibrary.Map_Find` _outparams "Team1") "NewEnumerator1")
  (`self.AddAllPlayersToTeam` (`local.Result`) (`BlueprintMapLibrary.Map_Find` _outparams "Team2") "NewEnumerator2")
  (return (`local.Result`)))

(fn `OnRep_GameStatus`
  (`self.GameStatusDispatcher` (`self.GameStatus`)))

(fn `RemovePlayerFromTeam`
  (params (Team :type "/Game/Blueprints/Game/E_Teams Enum" :default "NewEnumerator0") (Player :type "/Game/Blueprints/Player/BP_PlayerState Object Reference"))
  (`/Engine/EditorBlueprintResources/StandardMacros.DecrementInt` (`self.NumPlayers`)
    (:`  `
      (bind (_players _array_index) (`self.FindArrayToAdd` Team))
      (bind (_team _players_2 _score) (break `/Game/Blueprints/Game/ST_TeamPlayers` _players))
      (`KismetArrayLibrary.Array_RemoveItem` _players_2 (`local.Player`))
      (`KismetArrayLibrary.Array_Set` (`self.Teams`) _array_index (make `/Game/Blueprints/Game/ST_TeamPlayers` _team _players_2 _score))
      (set `/Game/Blueprints/Player/BP_PlayerState.Team` "NewEnumerator0" (`local.Player`)))))

(fn `SelectTeamToAddPlayer`
  (params (PlayerId :type String))
  (returns (Team :type "/Game/Blueprints/Game/E_Teams Enum"))
  (locals (CurrentTeam :type "/Game/Blueprints/Game/E_Teams Enum") (CurrentLength :type Integer :default 0))
  (bind (_value _returnvalue) (`BlueprintMapLibrary.Map_Find` (`self.PlayerIdToTeam`) PlayerId))
  (bind (_team _players) (break `/Game/Blueprints/Game/ST_TeamPlayers` (`|GetArrayItem` (`self.Teams`))))
  (if (`KismetStringLibrary.EqualEqual_StrStr` (`KismetSystemLibrary.GetBuildConfiguration`) "Development")
    (set `local.CurrentTeam` _team)
    (set `local.CurrentLength` (`KismetArrayLibrary.Array_Length` _players))
    (for _array_element (`self.Teams`)
      (bind (_team_2 _players_2) (break `/Game/Blueprints/Game/ST_TeamPlayers` _array_element))
      (bind _returnvalue_2 (`KismetArrayLibrary.Array_Length` _players_2))
      (if (< _returnvalue_2 (`local.CurrentLength`))
        (set `local.CurrentTeam` _team_2)
        (set `local.CurrentLength` _returnvalue_2)))
    (return (`local.CurrentTeam`))
    (elif _returnvalue
      (return _value)
      (else
        (return "NewEnumerator0")))))

(fn `SetScoreToTeam`
  (params (Team :type "/Game/Blueprints/Game/E_Teams Enum" :default "NewEnumerator0") (Score :type Integer))
  (bind (_players _array_index) (`self.FindArrayToAdd` Team))
  (bind (_team _players_2) (break `/Game/Blueprints/Game/ST_TeamPlayers` _players))
  (`KismetArrayLibrary.Array_Set` (`self.Teams`) _array_index (make `/Game/Blueprints/Game/ST_TeamPlayers` _team _players_2 (`local.Score`)))
  (`self.ScoreUpdated` (`local.Team`))
  (return))

(fn `UserConstructionScript`)