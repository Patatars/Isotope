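; Player inventory component that holds items in a fixed-size slot array and tracks the selected slot.
; Server-only mutations fill the first empty slot, drop a droppable current item when full, and select the nearest remaining item after a drop.
; RepNotifies on the items and slot index fire update dispatchers on replication.
; On respawn, items in a particular state are re-interacted with the new pawn; storage check and death handler are stubs.
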(event `self.ReceiveBeginPlay`
  (`/Engine/EditorBlueprintResources/ActorComponentMacros.Switch Has Authority`
    (:`Authority`
      (`KismetArrayLibrary.Array_Resize` (`self.Items`) (`self.InventorySize`)))))

(fn `AddItem`
  (params (Item :type "/Game/Blueprints/Items/BP_Item Object Reference"))
  (returns (Success :type Boolean))
  (locals (ToDrop :type "/Game/Blueprints/Items/BP_Item Object Reference"))
  (bind (_slot _success) (`self.GetNearestEmptySlot`))
  (`/Engine/EditorBlueprintResources/ActorComponentMacros.Switch Has Authority`
    (:`Authority`
      (if _success
        (bind _success_2 (`self.SetItem` _slot (`local.Item`)))
        (return _success_2)
        (elif (`/Game/Blueprints/Items/BP_Item.CanBeDropped` (`self.GetCurrentSlot`))
          (bind _output_get (set `local.ToDrop` (`self.GetCurrentSlot`)))
          (bind _success_3 (`self.RemoveItemBySlot` (`KismetArrayLibrary.Array_Find` (`self.Items`) _output_get)))
          (if _success_3
            (`/Game/Blueprints/Items/BP_Item.Drop` (`local.ToDrop`) (0.0 0.0 0.0))
            (else
              (return false)))
          (else
            (return false)))))))

(fn `CanItemBeStored`
  (params (Item :type "/Game/Blueprints/Items/BP_Item Object Reference"))
  (returns (Can :type Boolean))
  (return false))

(fn `DropCurrentItem`
  (returns (Success :type Boolean))
  (bind _success (`self.DropItem` (`self.SlotIndex`)))
  (return _success))

(fn `DropItem`
  (params (Slot :type Integer))
  (returns (Success :type Boolean))
  (`/Engine/EditorBlueprintResources/ActorComponentMacros.Switch Has Authority`
    (:`Authority`
      (bind _success (`self.RemoveItemBySlot` Slot))
      (if _success
        (`self.SetSlotIndex` (`self.FindNearestItem` (`local.Slot`)))
        (return true)
        (else
          (return false))))))

(fn `FindNearestItem`
  (params (Slot :type Integer))
  (returns (NearestSlot :type Integer))
  (locals (BestIndex :type Integer :default -1) (BestOffset :type Integer :default 999))
  (for (_array_element _array_index) (`self.Items`)
    (if (and (<= (`KismetMathLibrary.Abs_Int` (- _array_index (`local.Slot`))) (`local.BestOffset`)) (`self.IsValidItem` _array_element))
      (bind _output_get (set `local.BestIndex` _array_index))
      (set `local.BestOffset` (`KismetMathLibrary.Abs_Int` (- _output_get (`local.Slot`))))))
  (return (`local.BestIndex`)))

(fn `GetCurrentSlot`
  (returns (Item :type "/Game/Blueprints/Items/BP_Item Object Reference"))
  (return (`|GetArrayItem` (`self.Items`) (`self.SlotIndex`))))

(fn `GetItems`
  (returns (Items :type "Array of /Game/Blueprints/Items/BP_Item Object Reference"))
  (return (`self.Items`)))

(fn `GetNearestEmptySlot`
  (returns (Slot :type Integer) (Success :type Boolean))
  (for (_array_element _array_index) (`self.Items`)
    (if (not (`self.IsValidItem` _array_element))
      (return _array_index true)))
  (return -1 false))

(fn `GetSlotIndex`
  (returns (SlotIndex :type Integer))
  (return (`self.SlotIndex`)))

(fn `HasItem`
  (params (Item :type "/Game/Blueprints/Items/BP_Item Object Reference"))
  (returns (Has :type Boolean))
  (return (`KismetArrayLibrary.Array_Contains` (`self.Items`) Item)))

(fn `IsValidItem`
  (params (Item :type "/Game/Blueprints/Items/BP_Item Object Reference"))
  (returns (Valid :type Boolean))
  (return (`KismetSystemLibrary.IsValid` Item)))

(fn `OnRep_Items`
  (`self.InventoryUpdated`))

(fn `OnRep_SlotIndex`
  (`self.SlotUpdated`))

(fn `PawnDead`)

(fn `PawnRespawn`
  (params (Pawn :type "Pawn Object Reference"))
  (`/Engine/EditorBlueprintResources/ActorComponentMacros.Switch Has Authority`
    (:`Authority`
      (for _array_element (`self.Items`)
        (`/Engine/EditorBlueprintResources/StandardMacros.IsValid` _array_element
          (:`Is Valid`
            (if (`|EnumEquality` (`/Game/Blueprints/Items/BP_Item.ItemState` _array_element) "NewEnumerator7")
              (`/Game/Blueprints/Items/BP_Item.Interact` _array_element (`local.Pawn`))))))
      (`self.SetSlotIndex` 0))))

(fn `RemoveItem`
  (params (Item :type "/Game/Blueprints/Items/BP_Item Object Reference"))
  (returns (Success :type Boolean))
  (bind _success (`self.RemoveItemBySlot` (`KismetArrayLibrary.Array_Find` (`self.Items`) Item)))
  (return _success))

(fn `RemoveItemBySlot`
  (params (Slot :type Integer))
  (returns (Success :type Boolean))
  (`/Engine/EditorBlueprintResources/ActorComponentMacros.Switch Has Authority`
    (:`Authority`
      (if (`KismetArrayLibrary.Array_IsValidIndex` (`self.Items`) Slot)
        (`KismetArrayLibrary.Array_Set` (`self.Items`) (`local.Slot`))
        (return true)
        (else
          (return false))))))

(fn `SetItem`
  (params (Slot :type Integer) (Item :type "/Game/Blueprints/Items/BP_Item Object Reference"))
  (returns (Success :type Boolean))
  (`/Engine/EditorBlueprintResources/ActorComponentMacros.Switch Has Authority`
    (:`Authority`
      (if (`KismetArrayLibrary.Array_IsValidIndex` (`self.Items`) Slot)
        (if (`self.IsValidItem` (`|GetArrayItem` (`self.Items`) (`local.Slot`)))
          (return false)
          (else
            (`KismetArrayLibrary.Array_Set` (`self.Items`) (`local.Slot`) (`local.Item`))
            (if (== (`self.SlotIndex`) (`local.Slot`))
              (`self.SlotIndexChanged`)
              (return true)
              (else
                (return true)))))
        (else
          (return false))))))

(fn `SetSlotIndex`
  (params (SlotIndex :type Integer))
  (if (and (`KismetMathLibrary.InRange_IntInt` SlotIndex 0 (`self.InventorySize`)) (`self.IsValidItem` (`|GetArrayItem` (`self.Items`) (`local.SlotIndex`))))
    (set `self.SlotIndex` (`local.SlotIndex`))
    (`self.SlotIndexChanged`)))