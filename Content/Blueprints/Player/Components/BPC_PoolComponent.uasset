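; BPC_PoolComponent is a player component that pools BP_DamageNumber floating damage actors for reuse.
; GetFloatingDamageActor pops the last pooled actor, or spawns a new one at the origin owned by the first player controller when the pool is empty.
; ReturnFloatingDamageActor adds a used actor back to the array, which acts as a stack with no size cap or pre-warming.
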(fn `GetFloatingDamageActor`
  (returns (Actor :type "/Game/Blueprints/Character/Components/BP_DamageNumber Object Reference"))
  (if (`KismetArrayLibrary.Array_IsEmpty` (`self.FloatingDamageActors`))
    (bind _returnvalue (`|SpawnActorFromClass` "/Game/Blueprints/Character/Components/BP_DamageNumber.BP_DamageNumber_C" (`KismetMathLibrary.MakeTransform` (0.0 0.0 0.0)) "Undefined" "MultiplyWithRoot" (`GameplayStatics.GetPlayerController` 0) (`GameplayStatics.GetPlayerCharacter` 0)))
    (return _returnvalue)
    (else
      (bind _output (`self.Pop` (`self.FloatingDamageActors`)))
      (return _output))))

(fn `LastIndex`
  (params (TargetArray :type "Array of /Game/Blueprints/Character/Components/BP_DamageNumber Object Reference (by ref)"))
  (returns (ReturnValue :type Integer))
  (return (- (`KismetArrayLibrary.Array_Length` TargetArray) 1)))

(fn `Pop`
  (params (Array :type "Array of /Game/Blueprints/Character/Components/BP_DamageNumber Object Reference"))
  (returns (Output :type "/Game/Blueprints/Character/Components/BP_DamageNumber Object Reference"))
  (locals (LocalEl :type "/Game/Blueprints/Character/Components/BP_DamageNumber Object Reference"))
  (set `local.LocalEl` (`|GetArrayItem` (`local.Array`) (`self.LastIndex` (`local.Array`))))
  (`KismetArrayLibrary.Array_Remove` (`local.Array`) (`self.LastIndex` (`local.Array`)))
  (return (`local.LocalEl`)))

(fn `ReturnFloatingDamageActor`
  (params (Actor :type "/Game/Blueprints/Character/Components/BP_DamageNumber Object Reference (by ref)"))
  (`KismetArrayLibrary.Array_Add` (`self.FloatingDamageActors`) Actor))