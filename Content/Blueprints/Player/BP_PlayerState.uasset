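; Player state Blueprint that tracks a player's team, score, kills and deaths as replicated values.
; Add functions share a by-reference helper that increments the chosen stat and forces a net update.
; RepNotify handlers fire change dispatchers for UI or other listeners, with the team dispatcher limited to remote instances.
; On remote instances, score changes also reach the cached BP_GameState along with the player's team.
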(event `self.ReceiveBeginPlay`
  (bind _asbp_game_state (cast `/Game/Blueprints/Game/BP_GameState` (`GameplayStatics.GetGameState`)))
  (set `self.GameState` _asbp_game_state))

(fn `Add`
  (params (Variable :type "Integer (by ref)") (Add :type Integer))
  (`|VariableSetRef` Variable (+ Variable Add))
  (`self.ForceNetUpdate`))

(fn `AddDeath`
  (params (Add :type Integer))
  (`self.Add` (`self.DeathCount`) Add))

(fn `AddKill`
  (params (Add :type Integer))
  (`self.Add` (`self.KillCount`) Add))

(fn `AddOwnScore`
  (params (Add :type Integer))
  (`self.Add` (`self.OwnScore`) Add))

(fn `GetDeathCount`
  (returns (DeathCount :type Integer))
  (return (`self.DeathCount`)))

(fn `GetKillCount`
  (returns (KillCount :type Integer))
  (return (`self.KillCount`)))

(fn `GetOwnScore`
  (returns (OwnScore :type Integer))
  (return (`self.OwnScore`)))

(fn `OnRep_DeathCount`
  (`self.DeathCountUpdated` (`self.DeathCount`)))

(fn `OnRep_KillCount`
  (`self.KillCountUpdated` (`self.KillCount`)))

(fn `OnRep_OwnScore`
  (`self.OwnScoreUpdated` (`self.OwnScore`))
  (`/Engine/EditorBlueprintResources/ActorMacros.Switch Has Authority`
    (:`Remote`
      (`/Game/Blueprints/Game/BP_GameState.ScoreUpdated` (`self.GameState`) (`self.Team`) (`self.OwnScore`)))))

(fn `OnRep_Team`
  (`/Engine/EditorBlueprintResources/ActorMacros.Switch Has Authority`
    (:`Remote`
      (`self.TeamChanged` (`self.Team`)))))

(fn `UserConstructionScript`)