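; Player controller for the Isotope shooter mode, handling client-side adaptive music, saved volume settings and HUD updates for score and hits.
; Clients apply saved sound-class volumes, then drive MS_Music through parameters following game status and win result.
; Dealing or taking hits switches music to a combat state until a three-second timer expires.
; The HUD shows server-counted hits as a percentage of client-counted hits, alongside the isotope score.
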(event `self.ReceiveBeginPlay`
  (`parent.ReceiveBeginPlay`)
  (`/Engine/EditorBlueprintResources/ActorMacros.Switch Has Authority`
    (:`Remote`
      (`GameplayStatics.SetBaseSoundMix` "/Game/Music/SCM_Master.SCM_Master")
      (bind _audiovalue (message `/Game/Blueprints/Interfaces/BPI_Menu.GetSaveAudioSettings` (`GameplayStatics.GetGameInstance`)))
      (`self.ApplyAudioSetting` _audiovalue)
      (bind _returnvalue (`GameplayStatics.CreateSound2D` "/Game/Music/MS_Music.MS_Music" 1.0 1.0 0.0 null))
      (bind _output_get (set `self.Audio` _returnvalue))
      (`AudioComponent.Play` _output_get 0.0))))

(event `self.OnGameStatusChanged`
  (params (Status :type "/Game/Blueprints/Game/E_GameStatus Enum" :default "NewEnumerator0"))
  (`parent.OnGameStatusChanged` Status)
  (set `self.GameStatus` Status)
  (`self.Audio`
    (:`then`
      (switch `/Game/Blueprints/Game/E_GameStatus` Status
        (:`NewEnumerator0`
          (`AudioParameterControllerInterface.SetIntParameter` (`self.Audio`) "State" (select `/Game/Blueprints/Game/E_GameStatus` (`self.GameStatus`) :`NewEnumerator1` 1 :`NewEnumerator4` 3) :!label _label))
        (:`NewEnumerator3`
          (goto _label))
        (:`NewEnumerator1`
          (goto _label))
        (:`NewEnumerator4`
          (goto _label))
        (:`NewEnumerator2`
          (`AudioParameterControllerInterface.SetBoolParameter` (`self.Audio`) "Win" (`self.IsWonTeam`))
          (`AudioParameterControllerInterface.SetTriggerParameter` (`self.Audio`) "OnGameEnd"))))
    (:`else`)))

(event `AddGuns`
  (message `/Game/Blueprints/Interfaces/BPI_ItemHolder.AddItem` (`self.K2_GetPawn`) null)
  (message `/Game/Blueprints/Interfaces/BPI_ItemHolder.AddItem` (`self.K2_GetPawn`) null))

(event `self.OnRep_CompletedHitted`
  (`parent.OnRep_CompletedHitted`)
  (`/Game/UI/HUD/UI_Shooter.UpdateCompletedHitPercent` (`self.ShooterWidgetUI`) (`self.CalculateCompleteHitPercent`)))

(event `self.OnOwnScoreUpdated`
  (params (Score :type Integer))
  (`/Game/UI/HUD/Isotope/UI_IsotopeBanner.SetIsotopeCount` (`/Game/UI/HUD/UI_Shooter.UI_IsotopeBanner` (`self.ShooterWidgetUI`)) Score))

(event `/Game/Blueprints/Interfaces/BPI_CombatObserver.Hitted`
  (params (PhysMaterial :type "PhysicalMaterial Object Reference"))
  (`/Engine/EditorBlueprintResources/ActorMacros.Switch Has Authority`
    (:`Authority`
      (`/Engine/EditorBlueprintResources/StandardMacros.IncrementInt` (`self.CompletedHitted`)))
    (:`Remote`
      (`|ExecutionSequence`
        (:`then_0`
          (`/Game/UI/HUD/UI_Shooter.OnHitted` (`self.ShooterWidgetUI`) (`PhysicalMaterial.SurfaceType` PhysMaterial))
          (`/Engine/EditorBlueprintResources/StandardMacros.IncrementInt` (`self.HittedOnClient`)
            (:`  `
              (`/Game/UI/HUD/UI_Shooter.UpdateCompletedHitPercent` (`self.ShooterWidgetUI`) (`self.CalculateCompleteHitPercent`)))))
        (:`then_1`
          (`self.Audio` :!label _label_2
            (:`then`
              (if (`KismetSystemLibrary.K2_IsValidTimerHandle` (`self.EndCombatTimer`))
                (`KismetSystemLibrary.K2_ClearAndInvalidateTimerHandle` (`self.EndCombatTimer`)))
              (switch `/Game/Blueprints/Game/E_GameStatus` (`self.GameStatus`)
                (:`NewEnumerator0`
                  _)
                (:`NewEnumerator3`
                  _)
                (:`NewEnumerator1`
                  _))
              (`AudioParameterControllerInterface.SetIntParameter` (`self.Audio`) "State" 2)
              (bind _returnvalue (`KismetSystemLibrary.K2_SetTimerDelegate` (delegate `CombatStopped`) 3.0))
              (set `self.EndCombatTimer` _returnvalue))
            (:`else`)))))))

(event `/Game/Blueprints/Interfaces/BPI_CombatObserver.WasHitten`
  (goto _label_2))

(event `CombatStopped`
  (switch `/Game/Blueprints/Game/E_GameStatus` (`self.GameStatus`)
    (:`NewEnumerator0`
      _)
    (:`NewEnumerator3`
      _)
    (:`NewEnumerator1`
      _))
  (`AudioParameterControllerInterface.SetIntParameter` (`self.Audio`) "State" 1))

(fn `ApplyAudioSetting`
  (params (Array :type "Array of Float (double-precision)"))
  (locals (ValueArrayElement :type "Float (double-precision)"))
  (for (_array_element _array_index) Array
    (set `local.ValueArrayElement` _array_element)
    (switch `int` _array_index
      (:`0`
        (`GameplayStatics.SetSoundMixClassOverride` "/Game/Music/SCM_Master.SCM_Master" "/Game/Music/SC_Master.SC_Master" (`local.ValueArrayElement`) 1.0 0.0))
      (:`1`
        (`GameplayStatics.SetSoundMixClassOverride` "/Game/Music/SCM_Master.SCM_Master" "/Game/Music/SC_Music.SC_Music" (`local.ValueArrayElement`) 1.0 0.0))
      (:`2`
        (`GameplayStatics.SetSoundMixClassOverride` "/Game/Music/SCM_Master.SCM_Master" "/Game/Music/SC_SFX.SC_SFX" (`local.ValueArrayElement`) 1.0 0.0))
      (:`3`
        (`GameplayStatics.SetSoundMixClassOverride` "/Game/Music/SCM_Master.SCM_Master" "/Game/Music/SC_UI.SC_UI" (`local.ValueArrayElement`) 1.0 0.0))
      (:`4`
        (`GameplayStatics.SetSoundMixClassOverride` "/Game/Music/SCM_Master.SCM_Master" "/Game/Music/SC_Voice.SC_Voice" (`local.ValueArrayElement`) 1.0 0.0)))))

(fn `CalculateCompleteHitPercent`
  (returns (Percent :type "Float (double-precision)"))
  (return (* (/ (`self.CompletedHitted`) (`self.HittedOnClient`)) 100.0)))

(fn `UserConstructionScript`
  (`parent.UserConstructionScript`))