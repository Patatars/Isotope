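; Networked item pickup that grants the overlapping actor an item class from a data table row and respawns on a timer.
; The server async-loads the class and controls collision, while clients async-load the mesh and handle hiding, bobbing, spinning and a timeline scale-in.
; The server's respawn delay adds the timeline length, so collision returns as the client animation ends.
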(event `self.ReceiveBeginPlay`
  (bind (_datatable _rowname) (break `DataTableRowHandle` (`self.Weapon Type`)))
  (bind _returnvalue (`|GetDataTableRow` _datatable _rowname)
    (:`then`
      (`/Engine/EditorBlueprintResources/ActorMacros.Switch Has Authority`
        (:`Authority`
          (bind (_staticmesh _spawnactor) (break `/Game/Blueprints/Pickups/ST_WeaponTableRow` _returnvalue))
          (bind _class (`|LoadAssetClass` _spawnactor)
            (:`Completed`
              (bind _asbp_item (castclass `/Game/Blueprints/Pickups/BP_Item` _class))
              (set `self.Weapon Class` _asbp_item))))
        (:`Remote`
          (bind _object (`|LoadAsset` _staticmesh)
            (:`Completed`
              (`StaticMeshComponent.SetStaticMesh` (`self.StaticMesh`) (cast `StaticMesh` _object :!pure true)))))))))

(event `self.SphereCollision.OnComponentBeginOverlap`
  (params (OverlappedComponent :type "PrimitiveComponent Object Reference") (OtherActor :type "Actor Object Reference") (OtherComp :type "PrimitiveComponent Object Reference") (OtherBodyIndex :type Integer) (bFromSweep :type Boolean) (SweepResult :type "HitResult Structure (by ref)"))
  (`self.HideItem`)
  (`KismetSystemLibrary.K2_SetTimerDelegate` (`|CreateDelegate` :!event `Enable Pickup`) (`self.CalculateSpawnTimeBasedOnAuthority`))
  (`/Engine/EditorBlueprintResources/ActorMacros.Switch Has Authority`
    (:`Authority`
      (message `/Game/Blueprints/Interfaces/BPI_ItemHolder.Add Item Class` OtherActor (`self.Weapon Class`))
      (`PrimitiveComponent.SetCollisionEnabled` (`self.SphereCollision`) "NoCollision"))))

(event `self.ReceiveTick`
  (params (DeltaSeconds :type "Float (single-precision)"))
  (`self.Spin` (1.0 1.0 1.0)))

(event `Enable Pickup`
  (`/Engine/EditorBlueprintResources/ActorMacros.Switch Has Authority`
    (:`Authority`
      (`PrimitiveComponent.SetCollisionEnabled` (`self.SphereCollision`) "QueryOnly"))
    (:`Remote`
      (`SceneComponent.SetHiddenInGame` (`self.StaticMesh`) false false)
      (bind (_direction _scalein) (`Timeline|SpawnIn` :!via `PlayFromStart`)
        (:`Update`
          (`self.Spin` (`KismetMathLibrary.Conv_DoubleToVector` _scalein)))
        (:`Finished`
          (`self.SetActorTickEnabled` true))))))

(fn `CalculateSpawnTimeBasedOnAuthority`
  (returns (ReturnValue :type "Float (double-precision)"))
  (bind _spawn_time (`self.Spawn Time`))
  (`/Engine/EditorBlueprintResources/ActorMacros.Switch Has Authority`
    (:`Authority`
      (return (+ _spawn_time (`TimelineComponent.GetTimelineLength` (`self.SpawnIn`)))))
    (:`Remote`
      (return _spawn_time))))

(fn `HideItem`
  (`/Engine/EditorBlueprintResources/ActorMacros.Switch Has Authority`
    (:`Authority`
      (`PrimitiveComponent.SetCollisionEnabled` (`self.SphereCollision`) "NoCollision"))
    (:`Remote`
      (`SceneComponent.SetHiddenInGame` (`self.StaticMesh`) true false)
      (`self.SetActorTickEnabled` false))))

(fn `Spin`
  (params (`New Transform Scale` :type "Vector Structure" :default (1.0 1.0 1.0)))
  (bind _returnvalue (`KismetSystemLibrary.GetGameTimeInSeconds`))
  (`SceneComponent.K2_SetRelativeTransform` (`self.StaticMesh`) (`KismetMathLibrary.MakeTransform` (`KismetMathLibrary.MakeVector` 0.0 0.0 (* (`KismetMathLibrary.Sin` (* _returnvalue 3.0)) 15.0)) (`KismetMathLibrary.MakeRotator` 0.0 0.0 (* _returnvalue 100.0)) `New Transform Scale`) false false))

(fn `UserConstructionScript`
  (`/Engine/EditorBlueprintResources/ActorMacros.Switch Has Authority`
    (:`Authority`
      (`self.SetActorTickEnabled` false))))