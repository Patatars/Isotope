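; Hitscan fire component for weapons, extending a parent fire component's server fire and client effect functions.
; On the server, it traces on the Camera channel from the weapon to the owning pawn's target location, ignoring that pawn, and applies weapon damage.
; On clients, it spawns a Niagara trail at the muzzle aimed at the target, plus an attached muzzle effect offset for the locally controlled player.
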(fn `Clients_PlayEffects`
  (bind _weaponowner (`self.weaponOwner`))
  (bind _weaponowner_2 (`self.weaponOwner`))
  (bind _returnvalue_location (`KismetMathLibrary.BreakTransform` (`SceneComponent.GetSocketTransform` (`/Game/Blueprints/Pickups/BP_ShooterWeaponBase.SelectWeaponMesh` _weaponowner_2) "Muzzle" "RTS_World")))
  (`parent.Clients_PlayEffects`)
  (bind _target (message `/Game/Blueprints/Interfaces/BPI_WeaponHolder.Get Weapon Target Location` (`/Game/Blueprints/Pickups/BP_ShooterWeaponBase.Pawn Owner` _weaponowner_2)))
  (bind _returnvalue (`NiagaraFunctionLibrary.SpawnSystemAtLocation` "/Game/Fx/ArrowTrail/FX/NS_ArrowTrail_Magic_3.NS_ArrowTrail_Magic_3" _returnvalue_location (`KismetMathLibrary.FindLookAtRotation` _returnvalue_location _target)))
  (`NiagaraComponent.SetVariableFloat` _returnvalue "Speed" 50.0)
  (`NiagaraFunctionLibrary.SpawnSystemAttached` "/Game/Fx/NS_B.NS_B" (`/Game/Blueprints/Pickups/BP_ShooterWeaponBase.SelectWeaponMesh` _weaponowner) "Muzzle" (`KismetMathLibrary.SelectVector` (-40.0 0.0 0.0) (0.0 0.0 0.0) (`Pawn.IsLocallyControlled` (`/Game/Blueprints/Pickups/BP_ShooterWeaponBase.Pawn Owner` _weaponowner))) (struct) "KeepRelativeOffset" true))

(fn `Server_ProcessFire`
  (bind _weaponowner (`self.weaponOwner`))
  (bind _weaponowner_2 (`self.weaponOwner`))
  (bind _pawn_owner (`/Game/Blueprints/Pickups/BP_ShooterWeaponBase.Pawn Owner` _weaponowner_2))
  (`parent.Server_ProcessFire`)
  (bind _target (message `/Game/Blueprints/Interfaces/BPI_WeaponHolder.Get Weapon Target Location` _pawn_owner))
  (bind (_outhit _returnvalue) (`KismetSystemLibrary.LineTraceSingle` (`Actor.K2_GetActorLocation` _weaponowner_2) _target "TraceTypeQuery2" false (`|MakeArray` _pawn_owner :!type "Actor Object Reference")))
  (if _returnvalue
    (`GameplayStatics.ApplyDamage` (`.HitActor` (`GameplayStatics.BreakHitResult` _outhit)) (`/Game/Blueprints/Pickups/BP_ShooterWeaponBase.Damage` _weaponowner) (`Pawn.GetController` (`/Game/Blueprints/Pickups/BP_ShooterWeaponBase.Pawn Owner` _weaponowner)) _weaponowner)))