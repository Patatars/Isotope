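; Weapon fire component that fires by spawning projectile actors.
; Its server fire override runs the parent logic, gets a target location from its owner and spawns the weapon's bullet class at the transform the weapon calculates for that target.
; The bullet takes the weapon's owner as owner and its pawn as instigator.
; The component's own spawn-transform function is an empty stub.
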(fn `Calculate Bullet Spawn Transform`
  (params (`Target Position` :type "Vector Structure"))
  (returns (NewParam :type "Transform Structure"))
  (return))

(fn `Server_ProcessFire`
  (bind _weaponowner (`self.weaponOwner`))
  (bind _weaponowner_2 (`self.weaponOwner`))
  (`parent.Server_ProcessFire`)
  (bind _target (message `/Game/Blueprints/Interfaces/BPI_WeaponHolder.Get Weapon Target Location` (`self.GetOwner`)))
  (`|SpawnActorFromClass` (`/Game/Blueprints/Pickups/BP_ShooterWeaponBase.Bullet Class` _weaponowner) (`/Game/Blueprints/Pickups/BP_ShooterWeaponBase.Calculate Bullet Spawn Transform` _weaponowner _target) "Undefined" "OverrideRootScale" (`Actor.GetOwner` _weaponowner_2) (`/Game/Blueprints/Pickups/BP_ShooterWeaponBase.Pawn Owner` _weaponowner_2)))