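; BP_FireComponent is a weapon component that handles firing in a networked game, split into server logic and client effects.
; Server_Fire runs ServerProcessFire, an empty stub here, then calls All_Fire, which plays effects only where the component lacks authority.
; Those effects message the weapon's owner to play the fire montage and add recoil, using data from WeaponOwner.
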(event `self.ReceiveBeginPlay`)

(event `Server_Fire`
  (`self.Server_ProcessFire`)
  (`self.All_Fire`))

(event `All_Fire`
  (`/Engine/EditorBlueprintResources/ActorComponentMacros.Switch Has Authority`
    (:`Remote`
      (`self.Clients_PlayEffects`))))

(fn `Clients_PlayEffects`
  (bind _returnvalue (`Actor.GetOwner` (`self.weaponOwner`)))
  (message `/Game/Blueprints/Interfaces/BPI_WeaponHolder.Play Firing Montage` _returnvalue (`.Fire_11_9D1DACA040BB9A612A40CC847A800AC8` (break `/Game/Blueprints/Pickups/ST_WeaponAnimations` (`/Game/Blueprints/Pickups/BP_ShooterWeaponBase.WeaponAnimationMontages` (`self.weaponOwner`)))))
  (message `/Game/Blueprints/Interfaces/BPI_WeaponHolder.Add Weapon Recoil` _returnvalue (`/Game/Blueprints/Pickups/BP_ShooterWeaponBase.Firing Recoil` (`self.weaponOwner`))))

(fn `Server_ProcessFire`)