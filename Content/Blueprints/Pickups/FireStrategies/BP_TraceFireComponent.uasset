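; Hitscan fire strategy component that gives weapons instant trace shots with damage and effects.
; Server fire gets a hit from the owning pawn's aim trace and applies point damage to the hit actor without checking for a blocking hit.
; Client effects attach a Niagara beam ending at the impact or trace end, plus a second fire effect, to the muzzle, and leave a short-lived decal on blocking hits.
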(fn `Clients_PlayEffects`
  (params (HitResult :type "HitResult Structure"))
  (locals (WeaponMesh :type "SkeletalMeshComponent Object Reference") (WeaponTargetLocation :type "Vector Structure" :default (0.0 0.0 0.0)) (HitResult :type "HitResult Structure"))
  (bind (_bblockinghit _binitialoverlap _time _distance _location _impactpoint _normal _impactnormal _physmat _hitactor _hitcomponent _hitbonename _bonename _hititem _elementindex _faceindex _tracestart _traceend) (`GameplayStatics.BreakHitResult` (`local.HitResult`)))
  (bind (_bblockinghit_2 _binitialoverlap_2 _time_2 _distance_2 _location_2 _impactpoint_2 _normal_2 _impactnormal_2) (`GameplayStatics.BreakHitResult` (`local.HitResult`)))
  (`parent.Clients_PlayEffects` HitResult)
  (set `local.WeaponMesh` (`/Game/Blueprints/Pickups/BP_ShooterWeaponBase.SelectWeaponMesh` (`self.weaponOwner`)))
  (set `local.WeaponTargetLocation` (`KismetMathLibrary.SelectVector` _impactpoint _traceend _bblockinghit))
  (bind _returnvalue (`NiagaraFunctionLibrary.SpawnSystemAttached` (`self.Effect`) (`local.WeaponMesh`) "Muzzle" (0.0 0.0 0.0) (struct) "KeepRelativeOffset" true))
  (`NiagaraComponent.SetVariableVec3` _returnvalue "BeamEnd" (`local.WeaponTargetLocation`))
  (`NiagaraFunctionLibrary.SpawnSystemAttached` "/Game/Fx/NS_Fire1.NS_Fire1" (`/Game/Blueprints/Pickups/BP_ShooterWeaponBase.SelectWeaponMesh` (`self.weaponOwner`)) "Muzzle" (0.0 0.0 0.0) (struct) "KeepRelativeOffset" true)
  (if _bblockinghit_2
    (`GameplayStatics.SpawnDecalAtLocation` "/Game/Fx/Material/M_Master/M_Decal.M_Decal" (10.0 10.0 10.0) (`local.WeaponTargetLocation`) (`KismetMathLibrary.ComposeRotators` (`KismetMathLibrary.MakeRotFromZX` _impactnormal_2 (`KismetMathLibrary.GetUpVector` (struct))) (struct :`Roll` 90.0)) 5.0)))

(fn `Server_ProcessFire`
  (returns (HitResult :type "HitResult Structure"))
  (locals (Hit :type "HitResult Structure"))
  (bind _weaponowner (`self.weaponOwner`))
  (`parent.Server_ProcessFire`)
  (bind _hitresult (message `/Game/Blueprints/Interfaces/BPI_WeaponHolder.PerformAimTrace` (`/Game/Blueprints/Pickups/BP_ShooterWeaponBase.Pawn Owner` (`self.weaponOwner`))))
  (bind _output_get (set `local.Hit` _hitresult))
  (if true
    (`GameplayStatics.ApplyPointDamage` (`.HitActor` (`GameplayStatics.BreakHitResult` _output_get)) (`/Game/Blueprints/Pickups/BP_ShooterWeaponBase.Damage` _weaponowner) (`Actor.K2_GetActorLocation` (`self.weaponOwner`)) (`local.Hit`) (`Pawn.GetController` (`/Game/Blueprints/Pickups/BP_ShooterWeaponBase.Pawn Owner` _weaponowner)) _weaponowner)
    (return (`local.Hit`))
    (else
      (return (`local.Hit`)))))