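; BP_FireComponent is a weapon fire component that splits firing into server processing and client-side effects.
; Server_Fire calls ServerProcessFire, an empty stub here, and passes its result to All_Fire as the hit result.
; All_Fire runs ClientsPlayEffects only without authority, messaging the weapon's owner to play the firing montage and add recoil from the weapon's data.
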(event `self.ReceiveBeginPlay`)

(event `Server_Fire`
  (bind _hitresult (`self.Server_ProcessFire`))
  (`self.All_Fire` _hitresult))

(event `All_Fire`
  (params (HitResult :type "HitResult Structure"))
  (`/Engine/EditorBlueprintResources/ActorComponentMacros.Switch Has Authority`
    (:`Remote`
      (`self.Clients_PlayEffects` HitResult))))

(fn `Clients_PlayEffects`
  (params (HitResult :type "HitResult Structure"))
  (bind _returnvalue (`Actor.GetOwner` (`self.weaponOwner`)))
  (message `/Game/Blueprints/Interfaces/BPI_WeaponHolder.Play Firing Montage` _returnvalue (`.Fire_11_9D1DACA040BB9A612A40CC847A800AC8` (break `/Game/Blueprints/Pickups/ST_WeaponAnimations` (`/Game/Blueprints/Pickups/BP_Item.AnimationMontages` (`self.weaponOwner`)))))
  (message `/Game/Blueprints/Interfaces/BPI_WeaponHolder.Add Weapon Recoil` _returnvalue (`/Game/Blueprints/Pickups/BP_ShooterWeaponBase.Firing Recoil` (`self.weaponOwner`))))

(fn `Server_ProcessFire`
  (returns (HitResult :type "HitResult Structure"))
  (return))