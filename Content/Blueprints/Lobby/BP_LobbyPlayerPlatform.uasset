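; BP_LobbyPlayerPlatform is a lobby platform that displays one player's character at a fixed spawn point.
; SpawnCharacter stores the given player controller, destroys any existing character and spawns a BP_LobbyCharacter at the PlayerSpawnTransform component's world transform.
; Clear releases the player reference and destroys the character, freeing the platform.
; ShowFriendList and the construction script are empty stubs.
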(event `SpawnCharacter`
  (params (PC :type "PlayerController Object Reference"))
  (set `self.PC` PC)
  (bind _currentcharacter (`self.CurrentCharacter`)
    (:`then`
      (`self.K2_DestroyActor` _currentcharacter))
    (:`else`
      _))
  (bind _returnvalue (`|SpawnActorFromClass` "/Game/Blueprints/Lobby/BP_LobbyCharacter.BP_LobbyCharacter_C" (`SceneComponent.K2_GetComponentToWorld` (`self.PlayerSpawnTransform`)) "Undefined" "MultiplyWithRoot" null null))
  (set `self.CurrentCharacter` _returnvalue))

(event `Clear`
  (set `self.PC` null)
  (bind _currentcharacter (`self.CurrentCharacter`)
    (:`then`
      (`self.K2_DestroyActor` _currentcharacter)
      (set `self.CurrentCharacter` null))
    (:`else`)))

(fn `ShowFriendList`
  (params (show :type Boolean)))

(fn `UserConstructionScript`)