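; Player controller for the main menu lobby, bridging the UI with the Lobby and Matchmaking subsystems over a slowly rotating view.
; Login leads to EOS matchmaking authentication, then creation of a three-member lobby.
; Members publish proofs as attributes, which the owner submits to start matchmaking after opening a socket.
; Socket events update lobby attributes that sync search status, format and SessionId, which triggers each member's join ticket request and session connection.
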(event `self.ReceiveBeginPlay`
  (`|ExecutionSequence`
    (:`then_0`
      (`GameplayStatics.PlaySound2D` "/Game/Music/Wav/Lobby.Lobby" 1.0 1.0 0.0 null null)
      (set `self.bShowMouseCursor` true)
      (`ActorComponent.SetActive` (`Pawn.GetMovementComponent` (`self.K2_GetPawn`)) false false)
      (bind _menu (message `/Game/Blueprints/Interfaces/BPI_Menu.ToggleOnMainMenu` (`GameplayStatics.GetGameInstance`)))
      (set `self.UI` _menu)
      (`WidgetBlueprintLibrary.SetInputMode_UIOnlyEx` self (`self.UI`) "DoNotLock" true))
    (:`then_1`
      (add `LobbySubsystem.OnLoginSuccess` (subsystem `LobbySubsystem`) (`|CreateDelegate` :!event `OnLoginSuccess`))
      (add `LobbySubsystem.OnLobbyCreated` (subsystem `LobbySubsystem`) (`|CreateDelegate` :!event `OnLobbyCreated`))
      (`LobbySubsystem.OnLobbyAttributeUpdated` (subsystem `LobbySubsystem`) "SearchStatus" (`|CreateDelegate` :!event `OnSearchStatusUpdated`))
      (`LobbySubsystem.OnLobbyAttributeUpdated` (subsystem `LobbySubsystem`) "SessionId" (`|CreateDelegate` :!event `OnSessionIdUpdated`))
      (`LobbySubsystem.OnLobbyAttributeUpdated` (subsystem `LobbySubsystem`) "MatchFormat" (`|CreateDelegate` :!event `OnMatchFormatUpdated`))
      (add `LobbySubsystem.OnLobbyJoined` (subsystem `LobbySubsystem`) (`|CreateDelegate` :!event `OnLobbyJoined`))
      (add `LobbySubsystem.OnDisplayNameReady` (subsystem `LobbySubsystem`) (`|CreateDelegate` :!event `OnDisplayNameReady`))
      (add `LobbySubsystem.OnLobbyMemberJoined` (subsystem `LobbySubsystem`) (`|CreateDelegate` :!event `OnLobbyMemberJoined`))
      (add `LobbySubsystem.OnLobbyMemberLeft` (subsystem `LobbySubsystem`) (`|CreateDelegate` :!event `OnMemberLeft`))
      (add `LobbySubsystem.OnLobbyLeaderChanged` (subsystem `LobbySubsystem`) (`|CreateDelegate` :!event `OnLobbyLeaderChanged`))
      (add `LobbySubsystem.OnLobbyLeft` (subsystem `LobbySubsystem`) (`|CreateDelegate` :!event `OnLobbyLeft`))
      (add `LobbySubsystem.OnError` (subsystem `LobbySubsystem`) (delegate `OnError`))
      (add `MatchmakingSubsystem.OnError` (subsystem `MatchmakingSubsystem`) (`|CreateDelegate` :!event `OnError`)))
    (:`then_2`
      (if (not (`LobbySubsystem.IsLoggedIn` (subsystem `LobbySubsystem`)))
        (`LobbySubsystem.Login` (subsystem `LobbySubsystem`))))
    (:`then_3`
      ; UI binds
      (add `/Game/UI/Screens/UI_Lobby.OnSearchStatusSwitched` (`self.UI`) (`|CreateDelegate` :!event `OnSearchStatusSwitched`))
      (add `/Game/UI/Screens/UI_Lobby.OnMatchFormatChanged` (`self.UI`) (`|CreateDelegate` :!event `OnUIMatchFormatChanged`)))
    (:`then_4`
      (`LobbySubsystem.LeaveGameSession` :`self` (subsystem `LobbySubsystem`)))))

(event `self.ReceiveTick`
  (params (DeltaSeconds :type "Float (single-precision)"))
  (`self.SetControlRotation` (`KismetMathLibrary.MakeRotator` (.roll (`self.GetControlRotation`)) (.pitch (`self.GetControlRotation`)) (+ (.yaw (`self.GetControlRotation`)) (* DeltaSeconds 2.0)))))

(event `OnError`
  (params (Error :type "IsotopeError Structure (by ref)"))
  (bind (_method _error) (break `IsotopeError` Error))
  (message `/Game/Blueprints/Interfaces/BPI_Menu.ShowNotification` (`GameplayStatics.GetGameInstance`) (`KismetTextLibrary.Conv_StringToText` _method) (`KismetTextLibrary.Conv_StringToText` _error) 7.0))

(event `OnLobbyLeft`
  (params (Lobby :type "IsotopeLobbyBP Structure (by ref)"))
  (`/Game/UI/Screens/UI_Lobby.ClearMemberList` (`self.UI`))
  (`self.CreateLobby`))

(event `OnLobbyMemberJoined`
  (params (Lobby :type "IsotopeLobbyBP Structure (by ref)") (Member :type "IsotopeLobbyMemberBP Structure (by ref)"))
  (`/Game/UI/Screens/UI_Lobby.RefreshLobbyMembers` (`self.UI`) (`.Members` (break `IsotopeLobbyBP` Lobby))))

(event `OnLobbyLeaderChanged`
  (params (Lobby :type "IsotopeLobbyBP Structure (by ref)") (Member :type "IsotopeLobbyMemberBP Structure (by ref)"))
  (`self.RequestLobbyProof`)
  (if (`.bIsLocalMember` (break `IsotopeLobbyMemberBP` Member))
    (`/Game/UI/Screens/UI_Lobby.SetIsLobbyOwner` (`self.UI`) true)
    (`self.SetSearchStatusAttribute` "NewEnumerator0")))

(event `OnMatchFormatUpdated`
  (params (Attribute :type "IsotopeAttribute Structure (by ref)"))
  (`/Game/UI/Screens/UI_Lobby.SetMatchFormatValue` (`self.UI`) (cast `EMatchFormat` (`KismetMathLibrary.Conv_Int64ToByte` (`.AsInt` (break `IsotopeAttribute` Attribute))))))

(event `OnLoginSuccess`
  (params (AccountId :type String))
  (`LobbySubsystem.QueryExternalAuthCredential` (subsystem `LobbySubsystem`) (`|CreateDelegate` :!event `OnExternalAuthCredentials`)))

(event `OnMemberLeft`
  (params (Lobby :type "IsotopeLobbyBP Structure (by ref)") (Member :type "IsotopeLobbyMemberBP Structure (by ref)"))
  (`/Game/UI/Screens/UI_Lobby.RemoveLobbyMember` (`self.UI`) (`.AccountId` (break `IsotopeLobbyMemberBP` Member))))

(event `OnExternalAuthCredentials`
  (params (bSuccess :type Boolean) (CredentialType :type String) (Credential :type String))
  (if bSuccess
    (`MatchmakingSubsystem.AuthenticateEOS` (subsystem `MatchmakingSubsystem`) CredentialType Credential (`|CreateDelegate` :!event `OnAuthentificated`))))

(event `OnDisplayNameReady`
  (params (AccountId :type String) (DisplayName :type String))
  (`/Game/UI/Screens/UI_Lobby.AddNameToPlayer` (`self.UI`) AccountId DisplayName))

(event `OnLobbyJoined`
  (params (Lobby :type "IsotopeLobbyBP Structure (by ref)"))
  (bind ((`Attributes` _attributes)) (break `IsotopeLobbyBP` (`LobbySubsystem.GetCurrentLobby` (subsystem `LobbySubsystem`))))
  (`/Game/UI/Screens/UI_Lobby.ClearMemberList` (`self.UI`))
  (`/Game/UI/Screens/UI_Lobby.SetIsLobbyOwner` (`self.UI`) false)
  (`self.RequestLobbyProof`)
  (`self.OnSearchStatusUpdated` (`BlueprintMapLibrary.Map_Find` _attributes "SearchStatus"))
  (`self.OnMatchFormatUpdated` (`BlueprintMapLibrary.Map_Find` _attributes "MatchFormat")))

(event `OnLobbyCreated`
  (params (Lobby :type "IsotopeLobbyBP Structure (by ref)"))
  (`LobbySubsystem.SetLobbyAttribute` (subsystem `LobbySubsystem`) "Type" "Lobby")
  (`/Game/UI/Screens/UI_Lobby.SetIsLobbyOwner` (`self.UI`) true)
  (`self.SetMatchFormatAttribute` "THREE_V_THREE")
  (`self.SetSearchStatusAttribute` "NewEnumerator0")
  (`self.RequestLobbyProof`))

(event `OnAuthentificated`
  (params (bSuccess :type Boolean) (AuthData :type "GameAuthData Structure (by ref)"))
  (if bSuccess
    (set `self.Auth Data` AuthData)
    (`self.CreateLobby`)))

(event `OnLobbyMemberProofReceived`
  (params (bSuccess :type Boolean) (PUID :type String) (Proof :type String))
  (if bSuccess
    (`LobbySubsystem.SetMemberAttribute` (subsystem `LobbySubsystem`) "LobbyMemberProof" Proof)))

(event `OnWSEvent`
  (params (Event :type "MatchmakingSocketEvent Structure (by ref)"))
  (bind ((`Type` _type) (`SessionId` _sessionid)) (break `MatchmakingSocketEvent` Event))
  (`/Game/UI/Screens/UI_Lobby.SetRequestInProcess` (`self.UI`) false)
  (switch `EMatchmakingSocketEventType` _type
    (:`Queued`
      (`self.SetSearchStatusAttribute` "NewEnumerator1"))
    (:`ServerStarting`
      (`self.SetSearchStatusAttribute` "NewEnumerator2"))
    (:`SessionReady`
      (`LobbySubsystem.SetLobbyAttribute` (subsystem `LobbySubsystem`) "SessionId" _sessionid)
      (`self.SetSearchStatusAttribute` "NewEnumerator0")
      (`/Game/UI/Screens/UI_Lobby.SetIsSearching` (`self.UI`) false)
      (`MatchmakingSubsystem.DisconnectLobbySocket` (subsystem `MatchmakingSubsystem`)))
    (:`Cancelled`
      (`self.SetSearchStatusAttribute` "NewEnumerator0")
      (`MatchmakingSubsystem.DisconnectLobbySocket` (subsystem `MatchmakingSubsystem`)))
    (:`MatchmakingFailed`
      (`self.SetSearchStatusAttribute` "NewEnumerator3")
      (`/Game/UI/Screens/UI_Lobby.SetIsSearching` (`self.UI`) false)
      (`MatchmakingSubsystem.DisconnectLobbySocket` (subsystem `MatchmakingSubsystem`)))))

(event `OnSearchStatusUpdated`
  (params (Attribute :type "IsotopeAttribute Structure (by ref)"))
  (`/Game/UI/Screens/UI_Lobby.SetSearchStatus` (`self.UI`) (cast `/Game/Blueprints/Lobby/E_SearchStatus` (`KismetMathLibrary.Conv_Int64ToByte` (`.AsInt` (break `IsotopeAttribute` Attribute))))))

(event `OnSearchStatusSwitched`
  (params (Searching :type Boolean))
  (if Searching
    (if (`KismetStringLibrary.EqualEqual_StrStr` (`MatchmakingSubsystem.GetAuthenticatedPUID` (subsystem `MatchmakingSubsystem`)) (`.OwnerAccountId` (break `IsotopeLobbyBP` (`LobbySubsystem.GetCurrentLobby` (subsystem `LobbySubsystem`)))))
      (bind (_result _success) (`self.GetMembersNames`))
      (if _success
        (set `self.PendingMembers` _result)
        (`MatchmakingSubsystem.ConnectLobbySocket` :`self` (subsystem `MatchmakingSubsystem`) :`LobbyId` (`self.GetLobbyId`) :`ConnectionCompletion` (`|CreateDelegate` :!event `OnLobbySocketConnected`) :`EventHandler` (delegate `OnWSEvent`))
        (`/Game/UI/Screens/UI_Lobby.SetRequestInProcess` (`self.UI`) true)
        (else
          (`/Game/UI/Screens/UI_Lobby.SetIsSearching` (`self.UI`) false)))
      (else
        (`/Game/UI/Screens/UI_Lobby.SetIsSearching` (`self.UI`) false)))
    (else
      (`MatchmakingSubsystem.CancelMatchmaking` :`self` (subsystem `MatchmakingSubsystem`) :`LobbyId` (`self.GetLobbyId`))
      (`/Game/UI/Screens/UI_Lobby.SetRequestInProcess` (`self.UI`) true))))

(event `OnLobbySocketConnected`
  (params (bSuccess :type Boolean))
  (`/Game/UI/Screens/UI_Lobby.SetRequestInProcess` (`self.UI`) false)
  (if bSuccess
    (`MatchmakingSubsystem.StartMatchmaking` (subsystem `MatchmakingSubsystem`) (`self.GetLobbyId`) (`self.PendingMembers`) (`/Game/UI/Screens/UI_Lobby.GetMatchFormat` (`self.UI`)) (delegate `OnStartMatchmakingRepsonse`))
    (`/Game/UI/Screens/UI_Lobby.SetRequestInProcess` (`self.UI`) true)
    (else
      (`/Game/UI/Screens/UI_Lobby.SetIsSearching` (`self.UI`) false))))

(event `OnStartMatchmakingRepsonse`
  (params (bSuccess :type Boolean))
  (`/Game/UI/Screens/UI_Lobby.SetRequestInProcess` (`self.UI`) false)
  (if (not bSuccess)
    (`/Game/UI/Screens/UI_Lobby.SetIsSearching` (`self.UI`) false)))

(event `OnUIMatchFormatChanged`
  (params (MatchFormat :type "EMatchFormat Enum" :default "THREE_V_THREE"))
  (`self.SetMatchFormatAttribute` MatchFormat))

(event `OnSessionIdUpdated`
  (params (Attribute :type "IsotopeAttribute Structure (by ref)"))
  (bind (_key _type _asstring) (break `IsotopeAttribute` Attribute))
  (if (not (`KismetStringLibrary.IsEmpty` _asstring))
    (`MatchmakingSubsystem.RequestJoinTicket` (subsystem `MatchmakingSubsystem`) _asstring (delegate `OnJoinTicketRecieved`))
    (if (== (`LobbySubsystem.GetLocalAccountIdString` (subsystem `LobbySubsystem`)) (`.OwnerAccountId` (break `IsotopeLobbyBP` (`LobbySubsystem.GetCurrentLobby` (subsystem `LobbySubsystem`)))))
      (`LobbySubsystem.SetLobbyAttribute` (subsystem `LobbySubsystem`) "SessionId" "")
      (`/Game/UI/Screens/UI_Lobby.SetIsSearching` (`self.UI`) false))))

(event `OnJoinTicketRecieved`
  (params (bSuccess :type Boolean) (JoinTicket :type String))
  (if bSuccess
    (`LobbySubsystem.ConnectToSessionById` (subsystem `LobbySubsystem`) (`.AsString` (break `IsotopeAttribute` (`BlueprintMapLibrary.Map_Find` (`.Attributes` (break `IsotopeLobbyBP` (`LobbySubsystem.GetCurrentLobby` (subsystem `LobbySubsystem`)))) "SessionId"))) JoinTicket)))

(fn `CreateLobby`
  (`LobbySubsystem.CreateLobby` (subsystem `LobbySubsystem`) 3 "PublicAdvertised"))

(fn `GetLobbyId`
  (returns (LobbyId :type String))
  (return (`.LobbyId` (break `IsotopeLobbyBP` (`LobbySubsystem.GetCurrentLobby` (subsystem `LobbySubsystem`))))))

(fn `GetMembersNames`
  (returns (Result :type "Array of MatchmakingMemberProof Structure") (Success :type Boolean))
  (locals (Name :type "Array of MatchmakingMemberProof Structure"))
  (for _array_element (`LobbySubsystem.GetLobbyMembers` (subsystem `LobbySubsystem`))
    (bind (_accountid _displayname _bislocalmember _attributes) (break `IsotopeLobbyMemberBP` _array_element))
    (bind (_key _type _asstring) (break `IsotopeAttribute` (`BlueprintMapLibrary.Map_Find` _attributes "LobbyMemberProof")))
    (if (`KismetStringLibrary.IsEmpty` _asstring)
      (return _ false)
      (else
        (`KismetArrayLibrary.Array_Add` (`local.Name`) (make `MatchmakingMemberProof` _accountid _asstring)))))
  (return (`local.Name`) true))

(fn `RequestLobbyProof`
  (bind (_lobbyid _owneraccountid) (break `IsotopeLobbyBP` (`LobbySubsystem.GetCurrentLobby` (subsystem `LobbySubsystem`))))
  (`MatchmakingSubsystem.RequestLobbyMemberProof` (subsystem `MatchmakingSubsystem`) _lobbyid _owneraccountid (`|CreateDelegate` :!event `OnLobbyMemberProofReceived`)))

(fn `SetMatchFormatAttribute`
  (params (Index :type "EMatchFormat Enum" :default "THREE_V_THREE"))
  (`LobbySubsystem.SetLobbyAttributeInt` (subsystem `LobbySubsystem`) "MatchFormat" (`KismetMathLibrary.Conv_ByteToInt64` Index)))

(fn `SetSearchStatusAttribute`
  (params (Index :type "/Game/Blueprints/Lobby/E_SearchStatus Enum" :default "NewEnumerator0"))
  (`LobbySubsystem.SetLobbyAttributeInt` (subsystem `LobbySubsystem`) "SearchStatus" (`KismetMathLibrary.Conv_ByteToInt64` Index)))

(fn `UpdateMatchFormatStatus`
  (params (IsotopeLobbyBP :type "IsotopeLobbyBP Structure (by ref)"))
  (`/Game/UI/Screens/UI_Lobby.SetMatchFormatValue` (`self.UI`) (select `int` (`.AsInt` (break `IsotopeAttribute` (`BlueprintMapLibrary.Map_Find` (`.Attributes` (break `IsotopeLobbyBP` IsotopeLobbyBP)) "MatchFormat"))) :`0` "THREE_V_THREE" :`1` "ONE_V_ONE" :!type "EMatchFormat Enum")))

(fn `UserConstructionScript`)