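; BP_PartyManager handles automatic user login and online party lobby creation.
; StartAutologin runs an async auto-login, then calls CreatePartyLobby on success or quits the game on failure.
; CreatePartyLobby creates an advanced session tagged as a Party type, sized by MaxPartySize with lobby voice chat requested, and prints the result on screen.
; SendPartyInvite is an empty stub.
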(event `self.SendPartyInvite`)

(event `self.CreatePartyLobby`
  (`.CreateAdvancedSession` (`|MakeArray` (`self.MakeLiteralSessionPropertyString` "SessionType" "Party")) (`GameplayStatics.GetPlayerController` 0) (`self.MaxPartySize`) true false
    (:`OnSuccess`
      (`KismetSystemLibrary.PrintString` "LobbyCreated" true true (struct :`G` 1.0 :`A` 1.0) 10.0))
    (:`OnFailure`
      (`KismetSystemLibrary.PrintString` "FailedToCreateLobby" true true (struct :`R` 1.0 :`A` 1.0) 10.0))))

(event `self.StartAutologin`
  (`KismetSystemLibrary.PrintString` "Hello")
  (`.AutoLoginUser`
    (:`OnSuccess`
      (`self.CreatePartyLobby`))
    (:`OnFailure`
      (`KismetSystemLibrary.QuitGame` null "Quit"))))