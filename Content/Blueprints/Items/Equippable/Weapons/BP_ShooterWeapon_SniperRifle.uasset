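; Sniper rifle weapon Blueprint that adds an aim mode on the secondary action.
; Starting the action calls StartAim, which, if the weapon can fire, zeroes aim variance and turns on the owning pawn's aim mode through an interface message.
; Ending it calls StopAim, which restores aim variance from the class defaults and turns aim mode off.
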(event `/Game/Blueprints/Items/BP_EquippableItem.OnSecondaryActionStarted`
  (`parent.OnSecondaryActionStarted`)
  (`self.StartAim`))

(event `/Game/Blueprints/Items/BP_EquippableItem.OnSecondaryActionEnded`
  (`parent.OnSecondaryActionEnded`)
  (`self.StopAim`))

(fn `StartAim`
  (if (`self.CanFire`)
    (set `self.Aim Variance` 0.0)
    (message `/Game/Blueprints/Interfaces/BPI_WeaponHolder.ToggleAimMode` (`self.Pawn Owner`) true)))

(fn `StopAim`
  (set `self.Aim Variance` (defaults `/Game/Blueprints/Items/Equippable/Weapons/BP_ShooterWeapon_SniperRifle` "BP_ShooterWeapon_SniperRifle_C"))
  (message `/Game/Blueprints/Interfaces/BPI_WeaponHolder.ToggleAimMode` (`self.Pawn Owner`) false))

(fn `UserConstructionScript`
  (`parent.UserConstructionScript`))