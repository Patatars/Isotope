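; BP_JumpPowerUp is a collectable power-up that boosts the jump height of its owning pawn.
; ApplyEffect adds Value to the character movement component's JumpZVelocity, and RevertEffect subtracts the same Value.
; The component is fetched from the pawn through a GetCharacterMovementComponent message call.
; CanBeStored extends the parent check by also requiring the prospective owner to return a valid movement component.
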(event `self.ApplyEffect`
  (bind _component (message `/Game/Blueprints/Interfaces/BPI_ManagerAccessor.GetCharacterMovementComponent` (`self.Pawn Owner`)))
  (set `CharacterMovementComponent.JumpZVelocity` (+ (`CharacterMovementComponent.JumpZVelocity` _component) (`self.Value`)) _component))

(event `self.RevertEffect`
  (bind _component (message `/Game/Blueprints/Interfaces/BPI_ManagerAccessor.GetCharacterMovementComponent` (`self.Pawn Owner`)))
  (set `CharacterMovementComponent.JumpZVelocity` (- (`CharacterMovementComponent.JumpZVelocity` _component) (`self.Value`)) _component))

(fn `CanBeStored`
  (params (Owner :type "Actor Object Reference"))
  (returns (Can :type Boolean))
  (bind _component (message `/Game/Blueprints/Interfaces/BPI_ManagerAccessor.GetCharacterMovementComponent` Owner))
  (return (and (`parent.CanBeStored` (`local.Owner`)) (`KismetSystemLibrary.IsValid` _component))))

(fn `UserConstructionScript`
  (`parent.UserConstructionScript`))