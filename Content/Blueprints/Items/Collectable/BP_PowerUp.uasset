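; BP_PowerUp is a base collectable for timed power-ups, with empty ApplyEffect and RevertEffect events as hooks for specific effects.
; On pickup it calls the parent logic, then, on authority only, registers itself with the pawn owner's collectable manager via GetCollectableManagerMessage and applies the effect.
; A timer set to LifeTime then reverts the effect and destroys the actor.
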(event `self.OnPickedUp`
  (`parent.OnPickedUp`)
  (`/Engine/EditorBlueprintResources/ActorMacros.Switch Has Authority`
    (:`Authority`
      (bind _manager (message `/Game/Blueprints/Interfaces/BPI_ManagerAccessor.GetCollectableManager` (`self.Pawn Owner`)))
      (`/Game/Blueprints/Character/Components/BPC_CollectableManager.AddItem` _manager self)
      (`self.ApplyEffect`)
      (`KismetSystemLibrary.K2_SetTimerDelegate` (delegate `EndOfPowerUp`) (`self.LifeTime`)))))

(event `ApplyEffect`)

(event `EndOfPowerUp`
  (`self.RevertEffect`)
  (`self.K2_DestroyActor`))

(event `RevertEffect`)

(fn `UserConstructionScript`
  (`parent.UserConstructionScript`))