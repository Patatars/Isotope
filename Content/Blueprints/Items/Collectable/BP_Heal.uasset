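; BP_Heal is a collectable pickup that restores health to the pawn that picks it up.
; On pickup, the server calls Heal on the owner's health manager, fetched through GetHealthManagerMessage, then destroys the actor.
; CanBeStored extends the parent check by requiring a valid health manager that is not already full.
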(event `self.OnPickedUp`
  (`/Engine/EditorBlueprintResources/ActorMacros.Switch Has Authority`
    (:`Authority`
      (bind _manager (message `/Game/Blueprints/Interfaces/BPI_ManagerAccessor.GetHealthManager` (`self.Pawn Owner`)))
      (`/Game/Blueprints/Character/Components/BPC_HealthManager.Heal` _manager (`self.Heal`))
      (`self.K2_DestroyActor`))))

(fn `CanBeStored`
  (params (Owner :type "Actor Object Reference"))
  (returns (Can :type Boolean))
  (bind _manager (message `/Game/Blueprints/Interfaces/BPI_ManagerAccessor.GetHealthManager` Owner))
  (return (and (`KismetSystemLibrary.IsValid` _manager) (not (`/Game/Blueprints/Character/Components/BPC_HealthManager.IsFull` _manager)) (`parent.CanBeStored` (`local.Owner`)))))

(fn `UserConstructionScript`
  (`parent.UserConstructionScript`))