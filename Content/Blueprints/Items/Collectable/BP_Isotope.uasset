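; BP_Isotope is a collectable isotope item that reports pickups and losses to the game mode.
; It extends the parent's picked-up and dropped-down events, calling the parent logic first.
; On authority only, it gets the owning pawn's player state and sends the game mode a collected or loosed message with a count of one.
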(event `self.OnPickedUp`
  (`parent.OnPickedUp`)
  (`/Engine/EditorBlueprintResources/ActorMacros.Switch Has Authority`
    (:`Authority`
      (bind _playerstate (message `/Game/Blueprints/Interfaces/BPI_TeamPlayer.GetPlayerState` (`self.Pawn Owner`)))
      (message `/Game/Blueprints/Interfaces/BPI_IsotopeGameMode.IsotopeCollected` (`GameplayStatics.GetGameMode`) _playerstate 1))))

(event `self.OnDroppedDown`
  (`parent.OnDroppedDown`)
  (`/Engine/EditorBlueprintResources/ActorMacros.Switch Has Authority`
    (:`Authority`
      (bind _playerstate (message `/Game/Blueprints/Interfaces/BPI_TeamPlayer.GetPlayerState` (`self.Pawn Owner`)))
      (message `/Game/Blueprints/Interfaces/BPI_IsotopeGameMode.IsotopeLoosed` (`GameplayStatics.GetGameMode`) _playerstate 1))))

(fn `UserConstructionScript`)