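; Base weapon fire-strategy component that processes shots and plays firing feedback, with an empty ServerProcessFire stub for the hit calculation.
; Server_Fire applies seeded aim-cone variance on authority and sends hits to All_Fire; its remote branch calls FireOwner with unvaried direction for prediction.
; All_Fire plays effects only on remote, non-locally-controlled pawns, avoiding repeats of predicted effects.
; Effects cover montage, recoil, character-hit notifications and semi-auto refire cooldown display.
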(event `self.ReceiveBeginPlay`)

(event `FireOwner`
  (params (From :type "Vector Structure") (Direction :type "Vector Structure"))
  ;[0.1871 1 0] Fire prediction
  (bind _hitresult (`self.Server_ProcessFire` From Direction))
  (`self.Clients_PlayEffects` _hitresult))

(event `Server_Fire`
  (params (RandomStream :type "RandomStream Structure") (From :type "Vector Structure") (Direction :type "Vector Structure"))
  ;[1 0 0] Calculate Fire
  (set `self.Random Stream` RandomStream)
  (bind _returnvalue (`self.GetDirectionVectorWithAimVariance` Direction))
  (`/Engine/EditorBlueprintResources/ActorComponentMacros.Switch Has Authority`
    (:`Authority`
      (bind _hitresult (`self.Server_ProcessFire` From _returnvalue))
      (`self.All_Fire` _hitresult))
    (:`Remote`
      (`self.FireOwner` From Direction))))

(event `All_Fire`
  (params (HitResult :type "Array of HitResult Structure"))
  ;[0 0.1041 1] Fire effects
  (`/Engine/EditorBlueprintResources/ActorComponentMacros.Switch Has Authority`
    (:`Remote`
      (if (not (`Pawn.IsLocallyControlled` (`/Game/Blueprints/Items/BP_Item.Pawn Owner` (`self.weaponOwner`))))
        (`self.Clients_PlayEffects` HitResult)))))

(fn `Clients_PlayEffects`
  (params (HitResult :type "Array of HitResult Structure"))
  (bind _pawn_owner (`/Game/Blueprints/Items/BP_Item.Pawn Owner` (`self.weaponOwner`)))
  (message `/Game/Blueprints/Interfaces/BPI_WeaponHolder.Play Firing Montage` _pawn_owner (`.Fire_11_9D1DACA040BB9A612A40CC847A800AC8` (break `/Game/Blueprints/Items/Equippable/ST_WeaponAnimations` (`/Game/Blueprints/Items/BP_Item.AnimationMontages` (`self.weaponOwner`)))) (`self.MontagePlayRate`))
  (message `/Game/Blueprints/Interfaces/BPI_WeaponHolder.Add Weapon Recoil` _pawn_owner (`/Game/Blueprints/Items/Equippable/BP_ShooterWeaponBase.Firing Recoil` (`self.weaponOwner`)))
  (for _array_element (`local.HitResult`)
    (bind (_bblockinghit _binitialoverlap _time _distance _location _impactpoint _normal _impactnormal _physmat _hitactor) (`GameplayStatics.BreakHitResult` _array_element))
    (if (`GameplayStatics.ObjectIsA` _hitactor "/Game/Blueprints/Character/BP_ShooterCharacter.BP_ShooterCharacter_C")
      (`self.HitDispatcher`)
      (message `/Game/Blueprints/Interfaces/BPI_CombatObserver.Hitted` (`Pawn.GetController` (`/Game/Blueprints/Items/BP_Item.Pawn Owner` (`self.weaponOwner`))) _physmat)))
  (if (not (`/Game/Blueprints/Items/Equippable/BP_ShooterWeaponBase.Full Auto` (`self.weaponOwner`)))
    (message `/Game/Blueprints/Interfaces/BPI_WeaponHolder.ShowRefireCooldown` (`Pawn.GetController` (`/Game/Blueprints/Items/BP_Item.Pawn Owner` (`self.weaponOwner`))) (`/Game/Blueprints/Items/Equippable/BP_ShooterWeaponBase.Refire Rate` (`self.weaponOwner`)))))

(fn `GetDirectionVectorWithAimVariance`
  (params (Direction :type "Vector Structure (by ref)"))
  (returns (ReturnValue :type "Vector Structure"))
  (if (== (`/Game/Blueprints/Items/Equippable/BP_ShooterWeaponBase.Aim Variance` (`self.weaponOwner`)) 0.0)
    (return (`local.Direction`))
    (else
      (return (`KismetMathLibrary.RandomUnitVectorInConeInDegreesFromStream` (`self.Random Stream`) (`local.Direction`) (`/Game/Blueprints/Items/Equippable/BP_ShooterWeaponBase.Aim Variance` (`self.weaponOwner`)))))))

(fn `GetPawnOwner`
  (returns (`Pawn Owner` :type "Pawn Object Reference"))
  (return (`/Game/Blueprints/Items/BP_Item.Pawn Owner` (`self.weaponOwner`))))

(fn `Server_ProcessFire`
  (params (From :type "Vector Structure") (Direction :type "Vector Structure"))
  (returns (HitResult :type "Array of HitResult Structure"))
  (return))