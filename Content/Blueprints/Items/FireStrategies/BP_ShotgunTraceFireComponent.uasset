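; BP_ShotgunTraceFireComponent is a fire strategy component that gives a weapon shotgun-style multi-pellet trace fire.
; It overrides Server_ProcessFire to loop on the weapon owner's PelletsPerShot, applying random aim variance to the direction for each pellet.
; Each varied direction goes through the parent's fire processing, and the results are appended into one returned array.
; The event graph holds only disabled default events.
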(fn `Server_ProcessFire`
  (params (From :type "Vector Structure") (Direction :type "Vector Structure"))
  (returns (HitResult :type "Array of HitResult Structure"))
  (locals (Hit :type "HitResult Structure") (Res :type "Array of HitResult Structure"))
  (message `/Game/Blueprints/Interfaces/BPI_WeaponHolder.GetAimDirection` (`/Game/Blueprints/Items/BP_Item.Pawn Owner` (`self.weaponOwner`)))
  (for _ (range (+ (`/Game/Blueprints/Items/Equippable/BP_ShooterWeaponBase.PelletsPerShot ` (`self.weaponOwner`)) 1))
    (bind _returnvalue (`self.GetDirectionVectorWithAimVariance` (`local.Direction`)))
    (bind _hitresult (`parent.Server_ProcessFire` (`local.From`) _returnvalue))
    (`KismetArrayLibrary.Array_Append` (`local.Res`) _hitresult))
  (return (`local.Res`)))