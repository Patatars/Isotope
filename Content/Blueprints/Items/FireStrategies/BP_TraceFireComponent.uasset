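; Hitscan fire strategy component for weapons, resolving shots as line traces with server-side lag compensation.
; On authority it rewinds nearby shooter characters to a ping-based time, traces, restores them, then applies point damage scaled by a distance falloff curve.
; Client effects spawn a Niagara beam and muzzle effect at the weapon mesh, plus an impact decal on blocking hits.
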(fn `CalculateResultDamage`
  (params (HitLocation :type "Vector Structure"))
  (returns (ReturnValue :type "Float (double-precision)"))
  (return (* (`/Game/Blueprints/Items/Equippable/BP_ShooterWeaponBase.Damage` (`self.weaponOwner`)) (/ (`CurveFloat.GetFloatValue` (`/Game/Blueprints/Items/Equippable/BP_ShooterWeaponBase.DamageFallofCurve` (`self.weaponOwner`)) (`KismetMathLibrary.Vector_Distance` HitLocation (`Actor.K2_GetActorLocation` (`self.weaponOwner`)))) 100.0))))

(fn `Clients_PlayEffects`
  (params (HitResult :type "Array of HitResult Structure (by ref)"))
  (locals (WeaponMesh :type "SkeletalMeshComponent Object Reference") (WeaponTargetLocation :type "Vector Structure" :default (0.0 0.0 0.0)) (HitResult :type "HitResult Structure"))
  (`parent.Clients_PlayEffects` HitResult)
  (set `local.WeaponMesh` (`/Game/Blueprints/Items/Equippable/BP_ShooterWeaponBase.SelectWeaponMesh` (`self.weaponOwner`)))
  (for _array_element (`local.HitResult`)
    (bind (_bblockinghit _binitialoverlap _time _distance _location _impactpoint _normal _impactnormal _physmat _hitactor _hitcomponent _hitbonename _bonename _hititem _elementindex _faceindex _tracestart _traceend) (`GameplayStatics.BreakHitResult` _array_element))
    (set `local.WeaponTargetLocation` (`KismetMathLibrary.SelectVector` _impactpoint _traceend _bblockinghit))
    (bind _returnvalue (`NiagaraFunctionLibrary.SpawnSystemAttached` (`self.Effect`) (`local.WeaponMesh`) "Muzzle" (0.0 0.0 0.0) (struct) "KeepRelativeOffset" true))
    (`NiagaraComponent.SetVariableFloat` _returnvalue "Duration" (`/Game/Blueprints/Items/Equippable/BP_ShooterWeaponBase.TraceDuration` (`self.weaponOwner`)))
    (`NiagaraComponent.SetVariableVec3` _returnvalue "BeamEnd" (`local.WeaponTargetLocation`))
    (`NiagaraFunctionLibrary.SpawnSystemAttached` "/Game/Fx/NS_Fire1.NS_Fire1" (`/Game/Blueprints/Items/Equippable/BP_ShooterWeaponBase.SelectWeaponMesh` (`self.weaponOwner`)) "Muzzle" (0.0 0.0 0.0) (struct) "KeepRelativeOffset" true)
    (bind (_bblockinghit_2 _binitialoverlap_2 _time_2 _distance_2 _location_2 _impactpoint_2 _normal_2 _impactnormal_2) (`GameplayStatics.BreakHitResult` _array_element))
    (if _bblockinghit_2
      (`GameplayStatics.SpawnDecalAtLocation` "/Game/Fx/Material/M_Master/M_Decal.M_Decal" (10.0 10.0 10.0) (`local.WeaponTargetLocation`) (`KismetMathLibrary.ComposeRotators` (`KismetMathLibrary.MakeRotFromZX` _impactnormal_2 (`KismetMathLibrary.GetUpVector` (struct))) (struct :`Roll` 90.0)) 5.0))))

(fn `Server_ProcessFire`
  (params (From :type "Vector Structure") (Direction :type "Vector Structure"))
  (returns (HitResult :type "Array of HitResult Structure"))
  (locals (Hit :type "HitResult Structure") (RollbackAffectedActors :type "Array of Actor Object Reference"))
  (bind _actors (message `/Game/Blueprints/Interfaces/BPI_WeaponHolder.ActorsToBulletIgnore` (`/Game/Blueprints/Items/BP_Item.Pawn Owner` (`self.weaponOwner`))))
  (`/Engine/EditorBlueprintResources/ActorComponentMacros.Switch Has Authority`
    (:`Authority`
      (bind _affectedactors (`self.ServerRollbackCharacters` (`local.From`)))
      (set `local.RollbackAffectedActors` _affectedactors))
    (:`Remote`
      _))
  (bind _outhit (`KismetSystemLibrary.LineTraceSingle` From (+ From (* Direction 10000)) "TraceTypeQuery3" false _actors))
  (set `local.Hit` _outhit)
  (`/Engine/EditorBlueprintResources/ActorComponentMacros.Switch Has Authority`
    (:`Authority`
      (for _array_element (`local.RollbackAffectedActors`)
        (bind _component (message `/Game/Blueprints/Interfaces/BPI_ManagerAccessor.GetLagCompensationComponent` _array_element))
        (`/Game/Blueprints/Character/Components/BPC_LagCompensation.Restore` _component))
      (`GameplayStatics.ApplyPointDamage` (`.HitActor` (`GameplayStatics.BreakHitResult` (`local.Hit`))) (`self.CalculateResultDamage` (`.Location` (`GameplayStatics.BreakHitResult` (`local.Hit`)))) (`Actor.K2_GetActorLocation` (`self.weaponOwner`)) (`local.Hit`) (`Pawn.GetController` (`/Game/Blueprints/Items/Equippable/BP_ShooterWeaponBase.Pawn Owner` (`self.weaponOwner`))) (`self.weaponOwner`)))
    (:`Remote`
      _))
  (return (`|MakeArray` (`local.Hit`))))

(fn `ServerRollbackCharacters`
  (params (From :type "Vector Structure"))
  (returns (AffectedActors :type "Array of Actor Object Reference"))
  (bind _returnvalue (`PlayerState.GetPingInMilliseconds` (`Pawn.PlayerState` (`self.GetPawnOwner`))))
  (bind _outactors (`KismetSystemLibrary.SphereOverlapActors` From 99999.0 (`|MakeArray` "ObjectTypeQuery3" :!type "EObjectTypeQuery Enum") "/Game/Blueprints/Character/BP_ShooterCharacter.BP_ShooterCharacter_C" (`|MakeArray` (`self.GetPawnOwner`) :!type "Actor Object Reference")))
  (for _array_element _outactors
    (bind _component (message `/Game/Blueprints/Interfaces/BPI_ManagerAccessor.GetLagCompensationComponent` _array_element))
    (`/Game/Blueprints/Character/Components/BPC_LagCompensation.EnableAtTime` _component (- (`KismetSystemLibrary.GetGameTimeInSeconds`) (* _returnvalue 0.0005) (* _returnvalue 0.0001))))
  (return _outactors))