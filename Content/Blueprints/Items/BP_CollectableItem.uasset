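; BP_CollectableItem is an item Blueprint for collectables that can only be stored when a collectable manager allows it.
; Its CanBeStored override requires the parent check to pass, a valid collectable manager obtained from the owner through a message call, and that manager's CanItemBeCollected approval for this item.
; The event graph holds only disabled default events, and the construction script just calls the parent.
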(fn `CanBeStored`
  (params (Owner :type "Actor Object Reference"))
  (returns (Can :type Boolean))
  (bind _manager (message `/Game/Blueprints/Interfaces/BPI_ManagerAccessor.GetCollectableManager` Owner))
  (return (and (`parent.CanBeStored` (`local.Owner`)) (`KismetSystemLibrary.IsValid` _manager) (`/Game/Blueprints/Character/Components/BPC_CollectableManager.CanItemBeCollected` _manager self))))

(fn `UserConstructionScript`
  (`parent.UserConstructionScript`))