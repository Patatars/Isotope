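; Base Blueprint for equippable items that can be stored in inventory and dropped as loot, with empty action and reload events.
; Storing adds the item to the interactor's inventory; once stored, it hides loot effects, attaches its mesh to the pawn and notifies the equipment manager.
; Dropping reattaches the mesh to collision; authority places the actor before its owner, while remotes show the aura and custom-depth highlight, tinted by rarity.
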(event `self.OnStored`
  (`parent.OnStored`)
  (`ActorComponent.Deactivate` (`self.LootAura`))
  (`SceneComponent.SetHiddenInGame` (`self.DroppedFXRoot`) true true)
  (`PrimitiveComponent.SetRenderCustomDepth` (`self.Mesh`) false)
  (bind _pawn_owner (`self.Pawn Owner`)
    (:`then`
      (message `/Game/Blueprints/Interfaces/BPI_ItemHolder.Attach Item Mesh` _pawn_owner self (`self.Mesh`))
      (bind _manager (message `/Game/Blueprints/Interfaces/BPI_ManagerAccessor.GetEquipmentManager` (`self.Pawn Owner`)))
      (bind _output_get (set `self.PawnOwnerEquipmentManager` _manager))
      (`/Game/Blueprints/Character/Components/BPC_EquipmentManager.EnsureItemActivated` _output_get))
    (:`else`)))

(event `self.OnStartedDropping`
  (`self.Dropping`)
  (`parent.OnStartedDropping`))

(event `OnPrimaryActionStarted`
  ; API
)

(event `OnPrimaryActionEnded`
  ; API
)

(event `self.On Weapon Owner Destroyed`
  (params (KilledBy :type "Controller Object Reference"))
  (`self.OnPrimaryActionEnded`)
  (`self.OnSecondaryActionEnded`)
  (`parent.On Weapon Owner Destroyed` KilledBy))

(event `OnReloadRequested`
  ; API
)

(event `OnSecondaryActionStarted`
  ; API
)

(event `OnSecondaryActionEnded`
  ; API
)

(fn `CanBeStored`
  (params (Owner :type "Actor Object Reference"))
  (returns (Can :type Boolean))
  (message `/Game/Blueprints/Interfaces/BPI_ManagerAccessor.GetInventoryComponent` Owner)
  (return (and true (`parent.CanBeStored` (`local.Owner`)))))

(fn `Dropping`
  (bind _pawn_owner (`self.Pawn Owner`))
  (`SceneComponent.K2_AttachToComponent` (`self.Mesh`) (`self.Collision`) "None" "SnapToTarget" "SnapToTarget" "KeepWorld" false)
  (`SceneComponent.K2_SetRelativeTransform` (`self.Mesh`) (`KismetMathLibrary.MakeTransform` (0.0 0.0 0.0)) false false)
  (`|ExecutionSequence`
    (:`then_0`
      (`/Engine/EditorBlueprintResources/ActorMacros.Switch Has Authority`
        (:`Authority`
          (`self.K2_SetActorLocationAndRotation` (+ (`self.K2_GetActorLocation` _pawn_owner) (* (`self.GetActorForwardVector` _pawn_owner) 70) (* (`self.GetActorUpVector` _pawn_owner) 60)) (`KismetMathLibrary.MakeRotator` 0.0 0.0 (`KismetMathLibrary.RandomFloatInRange` 0.0 360.0)))
          (`self.ForceNetUpdate`))
        (:`Remote`
          (`ActorComponent.Activate` (`self.LootAura`) false)
          (`SceneComponent.SetHiddenInGame` (`self.DroppedFXRoot`) false true)
          (`PrimitiveComponent.SetRenderCustomDepth` (`self.Mesh`) true))))))

(fn `TryCommitStore`
  (params (Interactor :type "Pawn Object Reference"))
  (returns (Success :type Boolean))
  (bind _success (`parent.TryCommitStore` Interactor))
  (if _success
    (if (`|EnumEquality` (`self.ItemState`) "NewEnumerator7")
      (return true)
      (elif (`self.CanBeStored` (`local.Interactor`))
        (bind _component (message `/Game/Blueprints/Interfaces/BPI_ManagerAccessor.GetInventoryComponent` (`local.Interactor`)))
        (bind _success_2 (`/Game/Blueprints/Player/Components/BPC_InventoryComponent.AddItem` _component self))
        (return _success_2)))))

(fn `UpdateRarityVisuals`
  (params (VisualValues :type "/Game/Blueprints/Items/ST_RarityVisualInfo Structure"))
  (bind (_glowcolor _inventorybackground _stencil) (break `/Game/Blueprints/Items/ST_RarityVisualInfo` (`local.VisualValues`)))
  (`parent.UpdateRarityVisuals` VisualValues)
  (`PrimitiveComponent.SetCustomDepthStencilValue` (`self.Mesh`) _stencil)
  (`NiagaraComponent.SetVariableLinearColor` (`self.LootAura`) "Color" _glowcolor))

(fn `UserConstructionScript`
  (`parent.UserConstructionScript`))