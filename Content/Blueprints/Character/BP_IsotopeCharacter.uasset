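; Player character for an isotope-collecting shooter mode, extending a base shooter character with an overhead widget showing the isotope count.
; Clients cache the banner and update it from the PlayerState's score event, while the server caches the game mode.
; A role-gated Tick turns the counter toward the local player's pawn, and death hides it.
; Isotope pickup reporting and pistol/rifle granting exist only in disconnected nodes.
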(event `self.ReceiveBeginPlay`
  (`parent.ReceiveBeginPlay`)
  (`/Engine/EditorBlueprintResources/ActorMacros.Switch Has Authority`
    (:`Authority`
      (bind _asbp_isotope_game_mode (cast `/Game/Blueprints/Game/BP_IsotopeGameMode` (`self.BP_ShooterGameMode`)))
      (set `self.IsotopeGameMode` _asbp_isotope_game_mode))
    (:`Remote`
      (bind _asui_isotope_banner (cast `/Game/UI/HUD/Isotope/UI_IsotopeBanner` (`WidgetComponent.GetWidget` (`self.IsotopeCounter`))))
      (set `self.IsotopeBanner` _asui_isotope_banner)
      (`SceneComponent.SetHiddenInGame` (`self.IsotopeCounter`) false false))))

(event `self.ReceiveControllerChanged`
  (params (OldController :type "Controller Object Reference") (NewController :type "Controller Object Reference"))
  (`parent.ReceiveControllerChanged` OldController NewController)
  (`/Engine/EditorBlueprintResources/StandardMacros.IsValid` NewController
    (:`Is Valid`
      (`/Engine/EditorBlueprintResources/ActorMacros.Switch Has Authority`))))

(event `self.OnReplicatedPlayerState`
  (`parent.OnReplicatedPlayerState`)
  (add `/Game/Blueprints/Player/BP_PlayerState.OwnScoreUpdated` (`self.BP_PlayerState`) (delegate `OnIsotopeCountChanged`))
  (`self.OnIsotopeCountChanged` (`/Game/Blueprints/Player/BP_PlayerState.GetOwnScore` (`self.BP_PlayerState`))))

(event `self.ReceiveTick`
  (params (DeltaSeconds :type "Float (single-precision)"))
  (`parent.ReceiveTick` DeltaSeconds)
  (`/Game/Blueprints/Utils/BPM_PawnMacros.SwitchRole`
    (:`Other`
      (`SceneComponent.K2_SetWorldRotation` (`self.IsotopeCounter`) (`KismetMathLibrary.FindLookAtRotation` (`self.K2_GetActorLocation`) (`self.K2_GetActorLocation` (`Controller.K2_GetPawn` (`GameplayStatics.GetPlayerController` 0)))) false false))))

(event `OnIsotopeCountChanged`
  (params (Score :type Integer))
  (`/Engine/EditorBlueprintResources/ActorMacros.Switch Has Authority`
    (:`Remote`
      (bind _isotopebanner (`self.IsotopeBanner`)
        (:`then`
          (`/Game/UI/HUD/Isotope/UI_IsotopeBanner.SetIsotopeCount` _isotopebanner Score))
        (:`else`)))))

(fn `ClientsDie`
  (`SceneComponent.SetHiddenInGame` (`self.IsotopeCounter`) true false)
  (`parent.ClientsDie`))

(fn `OnRep_IsotopeNumber`)

(fn `SpawnAndAddItem`
  (params (Class :type "/Game/Blueprints/Items/BP_EquippableItem Class Reference") (Select :type Boolean) (CanBeDropped :type Boolean))
  (returns (Item :type "/Game/Blueprints/Items/BP_EquippableItem Object Reference"))
  (bind _returnvalue (`|SpawnActorFromClass` Class (`KismetMathLibrary.MakeTransform` (`self.K2_GetActorLocation`)) "AlwaysSpawn" "MultiplyWithRoot" (`self.GetController`) true (`local.Select`) "NewEnumerator2" (`local.CanBeDropped`) self))
  (`/Game/Blueprints/Interfaces/BPI_ItemHolder.AddItem` _returnvalue)
  (return _returnvalue))

(fn `UserConstructionScript`
  (`parent.UserConstructionScript`))