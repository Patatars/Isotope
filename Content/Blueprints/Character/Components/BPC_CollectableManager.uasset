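; BPC_CollectableManager is a character component that keeps a list of collected items.
; AddItem and RemoveItem edit the Items array, then refresh CountItems from its length.
; CountItems has a RepNotify, though its handler is currently empty.
; CanItemBeCollected always returns true, so the component applies no collection rules yet.
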(fn `AddItem`
  (params (Item :type "/Game/Blueprints/Items/BP_CollectableItem Object Reference"))
  (`KismetArrayLibrary.Array_Add` (`self.Items`) Item)
  (set `self.CountItems` (`KismetArrayLibrary.Array_Length` (`self.Items`))))

(fn `CanItemBeCollected`
  (params (Item :type "/Game/Blueprints/Items/BP_CollectableItem Object Reference"))
  (returns (Can :type Boolean))
  (return true))

(fn `OnRep_CountItems`)

(fn `RemoveItem`
  (params (Item :type "/Game/Blueprints/Items/BP_CollectableItem Object Reference"))
  (`KismetArrayLibrary.Array_RemoveItem` (`self.Items`) Item)
  (set `self.CountItems` (`KismetArrayLibrary.Array_Length` (`self.Items`))))