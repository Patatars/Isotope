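; BP_DamageNumber is a pooled actor that displays a floating damage number at a given world location.
; On BeginPlay it creates a UI_FloatingDamage widget, assigns it to its Damage component and adjusts the widget's offset and scale.
; InitDamage moves the actor and plays the widget with the damage amount and type.
; When the animation ends, the actor returns itself to the pool obtained through the player controller for reuse.
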(event `InitDamage`
  (params (Damage :type "Float (double-precision)") (DamageType :type "EPhysicalSurface Enum" :default "SurfaceType_Default") (Location :type "Vector Structure") (RightVector :type "Vector Structure") (UpVector :type "Vector Structure"))
  (`self.K2_SetActorLocation` Location)
  (`/Game/UI/HUD/UI_FloatingDamage.PLay` (`self.DamageWidget`) Damage DamageType))

(event `self.ReceiveBeginPlay`
  (bind _returnvalue (`|CreateWidget` "/Game/UI/HUD/UI_FloatingDamage.UI_FloatingDamage_C" (`GameplayStatics.GetPlayerController` 0)))
  (bind _output_get (set `self.DamageWidget` _returnvalue))
  (`WidgetComponent.SetWidget` (`self.Damage`) _output_get)
  (add `/Game/UI/HUD/UI_FloatingDamage.AnimEnded` (`self.DamageWidget`) (delegate `OnAnimationEnded`))
  (`Widget.SetRenderTranslation` (`self.DamageWidget`) (-100.0 -80.0))
  (`Widget.SetRenderScale` (`self.DamageWidget`) (0.7 0.7)))

(event `OnAnimationEnded`
  (bind _component (message `/Game/Blueprints/Interfaces/BPI_ManagerAccessor.GetPoolComponent` (`GameplayStatics.GetPlayerController` 0)))
  (`/Game/Blueprints/Player/Components/BPC_PoolComponent.ReturnFloatingDamageActor` _component self))

(fn `UserConstructionScript`)