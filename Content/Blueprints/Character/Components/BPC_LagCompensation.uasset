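; Server-side lag compensation component that rewinds the owner's tagged box hitboxes to a past moment.
; On authority, a looping timer records timestamped world transforms into a fixed-size ring buffer.
; EnableAtTime interpolates between the two snapshots bracketing the requested time, teleports the boxes there in absolute space and switches on their collision profile.
; Restore returns them to default relative transforms with collision off, and DisableAllCollisions deactivates the system.
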(event `self.ReceiveBeginPlay`
  (`/Engine/EditorBlueprintResources/ActorComponentMacros.Switch Has Authority`
    (:`Authority`
      (bind _output_get (set `self.Collisions` (`Actor.GetComponentsByTag` (`self.GetOwner`) "/Script/Engine.BoxComponent" (`self.CollisionsTag`))))
      (for _array_element _output_get
        (`KismetArrayLibrary.Array_Add` (`self.DefaultTransforms`) (`SceneComponent.GetRelativeTransform` _array_element)))
      (`KismetSystemLibrary.K2_SetTimer` null "SaveShapshot" (`self.SnapshotRate`) true)
      (set `self.Initialized` true))))

(event `self.ReceiveTick`
  (params (DeltaSeconds :type "Float (single-precision)")))

(event `EnableAtTime`
  (params (RewirndTime :type "Float (double-precision)"))
  (`/Engine/EditorBlueprintResources/ActorComponentMacros.Switch Has Authority`
    (:`Authority`
      (if (and (`self.Enabled`) (`self.Initialized`))
        (bind _snapshot (`self.GetSnapshotAtTime` RewirndTime))
        (if (`self.IsSnapshotValid` _snapshot)
          (for (_array_element _array_index) (`self.Collisions`)
            (bind (_timespamp _transforms) (break `/Game/Blueprints/Character/Snapshot/ST_HitBoxShapshot` _snapshot))
            (if (`KismetArrayLibrary.Array_IsValidIndex` _transforms _array_index)
              (`SceneComponent.SetAbsolute` _array_element true true true)
              (`SceneComponent.K2_SetWorldTransform` _array_element (`|GetArrayItem` _transforms _array_index) false true)
              (`PrimitiveComponent.SetCollisionProfileName` _array_element (`self.CollisionTurnedOn`) true))))))))

(event `Restore`
  (`/Engine/EditorBlueprintResources/ActorComponentMacros.Switch Has Authority`
    (:`Authority`
      (for (_array_element _array_index) (`self.Collisions`)
        (`PrimitiveComponent.SetCollisionProfileName` _array_element (`self.CollisionTurnedOff`) true)
        (`SceneComponent.SetAbsolute` _array_element false false false)
        (`SceneComponent.K2_SetRelativeTransform` _array_element (`|GetArrayItem` (`self.DefaultTransforms`) _array_index) false true)))))

(event `DisableAllCollisions`
  (`/Engine/EditorBlueprintResources/ActorComponentMacros.Switch Has Authority`
    (:`Authority`
      (set `self.Enabled` false)
      (for _array_element (`self.Collisions`)
        (`self.SetActive` _array_element false false)))))

(fn `GetNewSnapshotA`
  (params (RewindTime :type "Float (double-precision)") (CurrentSnapshot :type "/Game/Blueprints/Character/Snapshot/ST_HitBoxShapshot Structure (by ref)") (SnapshotA :type "/Game/Blueprints/Character/Snapshot/ST_HitBoxShapshot Structure (by ref)"))
  (returns (ResSnapshotA :type "/Game/Blueprints/Character/Snapshot/ST_HitBoxShapshot Structure (by ref)"))
  (bind _timespamp (break `/Game/Blueprints/Character/Snapshot/ST_HitBoxShapshot` CurrentSnapshot))
  (if (and (<= _timespamp (`local.RewindTime`)) (or (> _timespamp (`.Timespamp_3_75F120814AE3C0CC7AEE52B153F2EA22` (break `/Game/Blueprints/Character/Snapshot/ST_HitBoxShapshot` SnapshotA))) (not (`self.IsSnapshotValid` (`local.SnapshotA`)))))
    (return (`local.CurrentSnapshot`))
    (else
      (return (`local.SnapshotA`)))))

(fn `GetNewSnapshotB`
  (params (RewindTime :type "Float (double-precision)") (CurrentSnapshot :type "/Game/Blueprints/Character/Snapshot/ST_HitBoxShapshot Structure (by ref)") (SnapshotB :type "/Game/Blueprints/Character/Snapshot/ST_HitBoxShapshot Structure (by ref)"))
  (returns (ResSnapshotB :type "/Game/Blueprints/Character/Snapshot/ST_HitBoxShapshot Structure (by ref)"))
  (bind _timespamp (break `/Game/Blueprints/Character/Snapshot/ST_HitBoxShapshot` CurrentSnapshot))
  (if (and (>= _timespamp (`local.RewindTime`)) (or (< _timespamp (`.Timespamp_3_75F120814AE3C0CC7AEE52B153F2EA22` (break `/Game/Blueprints/Character/Snapshot/ST_HitBoxShapshot` SnapshotB))) (not (`self.IsSnapshotValid` (`local.SnapshotB`)))))
    (return (`local.CurrentSnapshot`))
    (else
      (return (`local.SnapshotB`)))))

(fn `GetSnapshotAtTime`
  (params (RewindTime :type "Float (double-precision)"))
  (returns (Snapshot :type "/Game/Blueprints/Character/Snapshot/ST_HitBoxShapshot Structure"))
  (locals (SnapshotA :type "/Game/Blueprints/Character/Snapshot/ST_HitBoxShapshot Structure" :default (struct :`Timespamp` -1.0 :`Transforms` "(())")) (SnapshotB :type "/Game/Blueprints/Character/Snapshot/ST_HitBoxShapshot Structure" :default (struct :`Timespamp` -1.0 :`Transforms` "(())")) (alpha :type "Float (double-precision)") (ResTransforms :type "Array of Transform Structure"))
  (for _array_element (`self.ShapshotBuffer`)
    (set `local.SnapshotA` (`self.GetNewSnapshotA` (`local.RewindTime`) _array_element (`local.SnapshotA`)))
    (set `local.SnapshotB` (`self.GetNewSnapshotB` (`local.RewindTime`) _array_element (`local.SnapshotB`))))
  (if (`self.IsSnapshotValid` (`local.SnapshotB`))
    (if (`self.IsSnapshotValid` (`local.SnapshotA`))
      (if (== (`.Timespamp_3_75F120814AE3C0CC7AEE52B153F2EA22` (break `/Game/Blueprints/Character/Snapshot/ST_HitBoxShapshot` (`local.SnapshotB`))) (`.Timespamp_3_75F120814AE3C0CC7AEE52B153F2EA22` (break `/Game/Blueprints/Character/Snapshot/ST_HitBoxShapshot` (`local.SnapshotA`))))
        (return (`local.SnapshotA`))
        (else
          (set `local.alpha` (/ (- (`local.RewindTime`) (`.Timespamp_3_75F120814AE3C0CC7AEE52B153F2EA22` (break `/Game/Blueprints/Character/Snapshot/ST_HitBoxShapshot` (`local.SnapshotA`)))) (- (`.Timespamp_3_75F120814AE3C0CC7AEE52B153F2EA22` (break `/Game/Blueprints/Character/Snapshot/ST_HitBoxShapshot` (`local.SnapshotB`))) (`.Timespamp_3_75F120814AE3C0CC7AEE52B153F2EA22` (break `/Game/Blueprints/Character/Snapshot/ST_HitBoxShapshot` (`local.SnapshotA`))))))
          (for (_ _array_index) (`self.Collisions`)
            (`KismetArrayLibrary.Array_Add` (`local.ResTransforms`) (`KismetMathLibrary.TLerp` (`|GetArrayItem` (`.Transforms_14_1B4D63D84A702E3D803C5A9A8C9A3A3D` (break `/Game/Blueprints/Character/Snapshot/ST_HitBoxShapshot` (`local.SnapshotA`))) _array_index) (`|GetArrayItem` (`.Transforms_14_1B4D63D84A702E3D803C5A9A8C9A3A3D` (break `/Game/Blueprints/Character/Snapshot/ST_HitBoxShapshot` (`local.SnapshotB`))) _array_index) (`local.alpha`))))
          (return (make `/Game/Blueprints/Character/Snapshot/ST_HitBoxShapshot` (`local.RewindTime`) (`local.ResTransforms`)))))
      (else
        (return (`local.SnapshotB`))))
    (else
      (return (`local.SnapshotA`)))))

(fn `IsSnapshotValid`
  (params (Snapshot :type "/Game/Blueprints/Character/Snapshot/ST_HitBoxShapshot Structure"))
  (returns (IsValid :type Boolean))
  (return (>= (`.Timespamp_3_75F120814AE3C0CC7AEE52B153F2EA22` (break `/Game/Blueprints/Character/Snapshot/ST_HitBoxShapshot` Snapshot)) 0.0)))

(fn `SaveShapshot`
  (locals (TransformsToSave :type "Array of Transform Structure"))
  (for _array_element (`self.Collisions`)
    (`KismetArrayLibrary.Array_Add` (`local.TransformsToSave`) (`SceneComponent.K2_GetComponentToWorld` _array_element)))
  (`KismetArrayLibrary.Array_Set` (`self.ShapshotBuffer`) (`self.SnaphsotIndex`) (make `/Game/Blueprints/Character/Snapshot/ST_HitBoxShapshot` (`KismetSystemLibrary.GetGameTimeInSeconds`) (`local.TransformsToSave`)) true)
  (set `self.SnaphsotIndex` (mod (+ (`self.SnaphsotIndex`) 1) (`self.SnapshotBufferSize`))))