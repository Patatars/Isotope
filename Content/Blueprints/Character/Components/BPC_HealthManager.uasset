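; Actor component that manages a character's health, handling damage, healing and death.
; Damage is doubled on Head surfaces, subtracted from HP clamped between zero and max, and broadcast through All_PlayHitFx for hit feedback.
; HP changes and death are written to RepNotify structs whose OnRep functions fire the HpChanged and Death dispatchers.
; An incrementing death counter makes each death a distinct replicated value.
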(event `ExecuteDamage`
  (params (Damage :type "Float (double-precision)") (HitLocation :type "Vector Structure") (HitNormal :type "Vector Structure") (isPointDamage :type Boolean) (InstigatedBy :type "Controller Object Reference") (DamagedPhysMaterial :type "PhysicalMaterial Object Reference"))
  (bind _outputdamage (`self.CalculateResultDamage` Damage DamagedPhysMaterial))
  (if (> (`self.CurrentHp`) 0.0)
    (`self.All_PlayHitFx` _outputdamage HitLocation HitNormal isPointDamage DamagedPhysMaterial)
    (bind _output_get (set `self.CurrentHp` (`self.CalculateNewHp` _outputdamage)))
    (set `self.HpUpdateInfo` (make `/Game/Blueprints/Character/Components/ST_HpUpdate` _output_get))
    (if (<= _output_get 0.0)
      (set `self.DeathInfo` (make `/Game/Blueprints/Character/Components/ST_DeathInfo` InstigatedBy (+ (`.DeathCounter_5_20C9503D429F7CE6D6A459B5BBE8F0A1` (break `/Game/Blueprints/Character/Components/ST_DeathInfo` (`self.DeathInfo`))) 1))))))

(event `All_PlayHitFx`
  (params (Damage :type "Float (double-precision)") (HitLocation :type "Vector Structure") (HitNormal :type "Vector Structure") (isPointDamage :type Boolean) (PhysMaterial :type "PhysicalMaterial Object Reference"))
  (`self.NotifyHit` Damage HitLocation HitNormal isPointDamage PhysMaterial))

(event `Heal`
  (params (Heal :type "Float (double-precision)"))
  (bind _output_get (set `self.CurrentHp` (`KismetMathLibrary.FClamp` (+ (`self.CurrentHp`) Heal) 0.0 (`self.MaxHP`))))
  (set `self.HpUpdateInfo` (make `/Game/Blueprints/Character/Components/ST_HpUpdate` _output_get true)))

(fn `CalculateNewHp`
  (params (Damage :type "Float (double-precision)"))
  (returns (Hp :type "Float (double-precision)"))
  (return (`KismetMathLibrary.FClamp` (- (`self.CurrentHp`) Damage) 0.0 (`self.MaxHP`))))

(fn `CalculateResultDamage`
  (params (InputDamage :type "Float (double-precision)") (PhysMaterial :type "PhysicalMaterial Object Reference"))
  (returns (OutputDamage :type "Float (double-precision)"))
  (return (* InputDamage (select `EPhysicalSurface` (`PhysicalMaterial.SurfaceType` PhysMaterial) :`SurfaceType_Default` 1.0 :`SurfaceType1` 2.0))))

(fn `IsFull`
  (returns (IsFull :type Boolean))
  (return (>= (`self.CurrentHp`) (`self.MaxHP`))))

(fn `OnRep_DeathInfo`
  (`self.Death` (`.Killer_2_82F4B6384997715DB8AA17B2C2B8A090` (break `/Game/Blueprints/Character/Components/ST_DeathInfo` (`self.DeathInfo`)))))

(fn `OnRep_HpUpdateInfo`
  (bind (_hp _raisedup) (break `/Game/Blueprints/Character/Components/ST_HpUpdate` (`self.HpUpdateInfo`)))
  (`self.HpChanged` _hp _raisedup (/ _hp (`self.MaxHP`))))