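; BP_HelpFunctions is a utility Blueprint that converts arrays between String and Text.
; StringToTextArray and TextToStringArray mirror each other, looping over the input and converting each element into a result array.
; Both collect results with AddUnique, so duplicate entries are dropped and the output can be shorter than the input.
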(fn `StringToTextArray`
  (params (Array :type "Array of String"))
  (returns (Array2 :type "Array of Text"))
  (locals (Res :type "Array of Text"))
  (for _array_element Array
    (`KismetArrayLibrary.Array_AddUnique` (`local.Res`) (`KismetTextLibrary.Conv_StringToText` _array_element)))
  (return (`local.Res`)))

(fn `TextToStringArray`
  (params (Array :type "Array of Text"))
  (returns (Array2 :type "Array of String"))
  (locals (Res :type "Array of String"))
  (for _array_element Array
    (`KismetArrayLibrary.Array_AddUnique` (`local.Res`) (`KismetTextLibrary.Conv_TextToString` _array_element)))
  (return (`local.Res`)))